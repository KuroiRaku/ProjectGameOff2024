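; BP_PatrolRoute is an enemy patrol route that exposes the points of a PatrolPath spline as world-space destinations.
; InCrementPatrolRouns steps PatrolIndex by Direction, flipping Direction at the first and last spline points so the route ping-pongs back and forth.
; GetSplinePositionInWorld returns the world location of the spline point at the current index.
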(event Custom|InCrementPatrolRouns
  (bind _output_get (Variables|Default|SetPatrol%20Index (+ (Variables|Default|GetPatrol%20Index) (Variables|Default|GetDirection))))
  (if (== _output_get (- (Spline|GetNumberOfSplinePoints (Variables|Default|GetPatrolPath)) 1))
    (Variables|Default|SetDirection -1)
    (elif (== (Variables|Default|GetPatrol%20Index) 0)
      (Variables|Default|SetDirection 1))))

(fn ConstructionScript)

(fn GetSplinePositioninWorld
  (return (Spline|GetLocationatSplinePoint (Variables|Default|GetPatrolPath) (Variables|Default|GetPatrol%20Index) "World")))