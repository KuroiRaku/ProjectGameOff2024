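; Enemy AI character that detects living players and non-hostage allies through pawn sensing and drives its blackboard state and alert level.
; A sighting sets the target and broadcasts one detection event with its location, while a retriggerable delay restarts with each sighting.
; When the delay expires, it clears the target, stores the last known position and changes alert state.
; SetTarget lets missions assign a target directly.
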(event OnSeePawn(PawnSensing)
  (params (Pawn :type Pawn%20Object%20Reference))
  (bind _self self)
  (bind _returnvalue (AI|GetAIController _self))
  (bind _returnvalue_2 (AI|GetBlackboard _returnvalue))
  (bind _isdead (CallFunction|IsDead))
  (if (not _isdead)
    (bind _asbp_player_character (Utilities|Casting|CastToBP_PlayerCharacter Pawn)
      (:then
        (bind _isdead_2 (Default|IsDead _asbp_player_character))
        (if (not _isdead_2)
          (bind _output_get (Variables|Default|SetTargetActor _asbp_player_character))
          (Variables|Ai|SetSeesPlayer? true)
          (Utilities|FlowControl|Sequence :!label _label ; This to reset the delay if we keep seeing the enemy
            (:then_0
              (AI|Components|Blackboard|SetValueasObject (AI|GetBlackboard (AI|GetAIController self)) (Variables|Ai|GetEnemy%20Key%20Name) (Variables|Default|GetTargetActor))
              (CallFunction|UpdateAlertState "NewEnumerator1")
              (if (not (Variables|Default|GetHasInformNPC))
                (Default|CallOnEnemyDetectedEvent (Transformation|GetActorLocation (Variables|Default|GetTargetActor)))
                (Variables|Default|SetHasInformNPC true)))
            (:then_1
              ;[1 1 1] If we lose player
              (Utilities|FlowControl|RetriggerableDelay 2.0)
              (bind _isdead_3 (CallFunction|IsDead))
              (if (not _isdead_3)
                (Utilities|IsValid _output_get
                  (:Is%20Valid
                    (Variables|Ai|SetSeesPlayer? false)
                    (bind _output_get_2 (Variables|Default|SetLastKnownPosition (Transformation|GetWorldLocation (Variables|/Script/Engine.Character|GetCapsuleComponent _output_get))))
                    (Variables|Default|SetTargetActor 0)
                    (Variables|Default|SetHasInformNPC false)
                    (AI|Components|Blackboard|SetValueasObject _returnvalue_2 (Variables|Ai|GetEnemy%20Key%20Name) (Variables|Default|GetTargetActor))
                    (AI|Components|Blackboard|SetValueasVector _returnvalue_2 (Variables|Default|GetLocation%20Key) _output_get_2)
                    (CallFunction|UpdateAlertState "NewEnumerator2"))))))))
      (:CastFailed
        (bind _asbp_ally_aicharacter (Utilities|Casting|CastToBP_AllyAICharacter Pawn))
        (bind _isdead_4 (Default|IsDead _asbp_ally_aicharacter))
        (if (not (or _isdead_4 (Variables|/Game/Characters/Ally/Blueprint/BP_AllyAICharacter.BP_AllyAICharacter_C|GetIsHostage _asbp_ally_aicharacter)))
          (Variables|Default|SetTargetActor _asbp_ally_aicharacter)
          (Variables|Ai|SetSeesPlayer? true)
          (goto _label))))))

(event Custom|SetTarget
  (params (Target :type BP%20Base%20Character%20Object%20Reference))
  ;[1 1 1] Use for mission
  (bind _output_get (Variables|Default|SetTargetActor Target))
  (AI|Components|Blackboard|SetValueasObject (AI|GetBlackboard (AI|GetAIController self)) (Variables|Ai|GetEnemy%20Key%20Name) _output_get)
  (CallFunction|UpdateAlertState "NewEnumerator1"))

(event EventBeginPlay
  (|CallParentFunction)
  (AI|Components|Blackboard|SetValueasEnum (AI|GetBlackboard (AI|GetAIController self)) (Variables|Ai|GetState%20Key%20Name) (Utilities|Enum|LiteralenumE_States "NewEnumerator0")) ; Setting Ai behaviour to IDLE when BP starts
)

(fn ConstructionScript
  (|CallParentFunction))