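; Behavior tree decorator for enemy AI that passes when the controlled pawn is at least a set distance from its target actor.
; PerformConditionCheckAI reads the target from the EnemyKey blackboard entry and measures the distance between both root component world locations.
; It returns true at or beyond DistanceToTarget and false when closer, with no validity check on the blackboard actor.
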(fn PerformConditionCheckAI
  (params (OwnerController :type AI%20Controller%20Object%20Reference) (ControlledPawn :type Pawn%20Object%20Reference))
  (if (>= (Math|Vector|Distance(Vector) (Transformation|GetWorldLocation (Variables|/Script/Engine.Actor|GetRootComponent ControlledPawn)) (Transformation|GetWorldLocation (Variables|/Script/Engine.Actor|GetRootComponent (AI|BehaviorTree|GetBlackboardValueasActor (Variables|Default|GetEnemyKey))))) (Variables|Default|GetDistanceToTarget))
    (return true)
    (else
      (return false))))