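; Behavior tree task that moves an ally AI character to a random nearby navigable location.
; It multiplies the pawn's forward vector component-wise by random X and Y values, offsets the pawn's location by the result, then samples a small navigable radius there.
; AIMoveTo drives the move and finishes the task with success or failure, failing also for non-ally pawns.
; It prints the chosen location and stops movement on abort.
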(event EventReceiveAbortAI
  (params (OwnerController :type AI%20Controller%20Object%20Reference) (ControlledPawn :type Pawn%20Object%20Reference))
  (AI|Navigation|StopMovement OwnerController))

(event EventReceiveExecuteAI
  (params (OwnerController :type AI%20Controller%20Object%20Reference) (ControlledPawn :type Pawn%20Object%20Reference))
  (bind _returnvalue (Math|Random|RandomFloatinRange -1e+03 1e+03))
  (Utilities|Casting|CastToBP_AllyAICharacter ControlledPawn
    (:then
      (bind _randomlocation (Class|NavigationSystemV1|GetRandomLocationinNavigableRadius (+ (Transformation|GetActorLocation ControlledPawn) (* (Math|Vector|MakeVector _returnvalue _returnvalue 1.0) (Transformation|GetActorForwardVector ControlledPawn))) 15.0 0 0))
      (Development|PrintString (Utilities|String|ToString(Vector) _randomlocation))
      (AI|AIMoveTo ControlledPawn _randomlocation 0 2.0 false
        (:OnSuccess
          (AI|BehaviorTree|FinishExecute true))
        (:OnFail
          (AI|BehaviorTree|FinishExecute false :!label _label))))
    (:CastFailed
      (goto _label))))