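; AI controller for ally characters that can join the player and take move commands.
; On possession of an ally or player character, it runs the ally behavior tree and seeds the blackboard location with the pawn's position.
; Perception updates write the enemy actor key, joining writes the player key, and GotoLocation stops movement and sets a new location for the tree.
; A delayed auto-join test is left unconnected.
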(event Custom|On%20Perception%20Actor%20Updated
  (params (Target%20Actor :type Actor%20Object%20Reference))
  (AI|Components|Blackboard|SetValueasObject (Variables|Default|GetBlackboard) (Variables|Default|GetEnemyActorKey) Target%20Actor))

(event Custom|Join%20Player
  (params (Player%20Character :type BP%20Player%20Character%20Object%20Reference))
  ;[1 1 1 1 37] Events
  ;;[1 1 1] Join Player
  (Variables|Default|SetJoinedPlayer true)
  (bind _output_get (Variables|Default|SetPlayerCharacter Player%20Character))
  (AI|Components|Blackboard|SetValueasObject (Variables|Default|GetBlackboard) (Variables|Default|GetPlayerKey) _output_get))

(event Custom|Go%20to%20Location
  (params (NewLocation :type Vector))
  ;[0.4225 0.5584 1 1 37] Commands
  ;;[1 1 1] Move Commands
  (AI|Navigation|StopMovement)
  (bind _output_get (Variables|Default|SetLocationToGo NewLocation))
  (AI|Components|Blackboard|SetValueasVector (Variables|Default|GetBlackboard) (Variables|Default|GetLocationKey) _output_get)
  (Variables|Default|SetHasLocationToGo true))

(event EventPossess
  (params (PossessedPawn :type Pawn%20Object%20Reference))
  ;[1 1 1 1 37] Run Behavior Tree When Possessed
  (bind _output_get (Variables|Default|SetPossesed%20Pawn PossessedPawn))
  (bind _asbp_ally_aicharacter (Utilities|Casting|CastToBP_AllyAICharacter _output_get)
    (:then
      (Variables|Default|SetPossesedAllyAICharacter _asbp_ally_aicharacter))
    (:CastFailed
      (bind _asbp_player_character (Utilities|Casting|CastToBP_PlayerCharacter _output_get))
      (Variables|Default|SetPossesedPlayerCharacter _asbp_player_character)))
  (AI|RunBehaviorTree "/Game/Characters/Ally/Blueprint/AllyAIBehaviorTree.AllyAIBehaviorTree")
  (bind _output_get_2 (Variables|Default|SetLocationToGo (Transformation|GetActorLocation (Variables|Default|GetPossesed%20Pawn))))
  (AI|Components|Blackboard|SetValueasVector (Variables|Default|GetBlackboard) (Variables|Default|GetLocationKey) _output_get_2))

(fn ConstructionScript)