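; Behavior tree task that moves an ally pawn to a location stored in a blackboard key.
; On execute it clears the controller's focus, then runs AI MoveTo toward the key's vector within an acceptance radius.
; Either move result clears HasLocationToGo on BP_AllyAIController and finishes with success or failure; a failed controller cast also fails.
; Aborting the task stops the controller's movement.
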(event EventReceiveExecuteAI
  (params (OwnerController :type AI%20Controller%20Object%20Reference) (ControlledPawn :type Pawn%20Object%20Reference))
  (AI|ClearFocus OwnerController)
  (bind _asbp_ally_aicontroller (Utilities|Casting|CastToBP_AllyAIController OwnerController)
    (:then
      (AI|AIMoveTo ControlledPawn (Class|BTFunctionLibrary|GetBlackboardValueasVector (Variables|Default|GetLocationKey)) 0 (Variables|Default|GetAcceptance%20Radius) false
        (:OnSuccess
          (Variables|/Game/Characters/Ally/Blueprint/BP_AllyAIController.BP_AllyAIController_C|SetHasLocationToGo _asbp_ally_aicontroller false)
          (AI|BehaviorTree|FinishExecute true))
        (:OnFail
          (Variables|/Game/Characters/Ally/Blueprint/BP_AllyAIController.BP_AllyAIController_C|SetHasLocationToGo _asbp_ally_aicontroller false)
          (AI|BehaviorTree|FinishExecute false :!label _label))))
    (:CastFailed
      (goto _label))))

(event EventReceiveAbortAI
  (params (OwnerController :type AI%20Controller%20Object%20Reference) (ControlledPawn :type Pawn%20Object%20Reference))
  (AI|Navigation|StopMovement OwnerController))