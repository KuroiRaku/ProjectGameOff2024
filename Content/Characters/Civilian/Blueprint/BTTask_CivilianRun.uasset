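; Behavior tree task that moves a civilian AI character in a run-away step.
; On execute it casts the pawn to BP_CivilianAICharacter, then RunAway issues an AI MoveTo 500 units away at the same height and finishes with its success or failure.
; The look-at rotation uses the civilian's own location as both start and target, so the destination always lies along world -X rather than away from a threat.
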(event Custom|RunAway
  (bind _as_bp_civilian_aicharacter (Variables|Default|GetAs%20BP%20Civilian%20AICharacter))
  (bind _as_bp_civilian_aicharacter_2 (Variables|Default|GetAs%20BP%20Civilian%20AICharacter))
  (bind _returnvalue (Transformation|GetActorLocation _as_bp_civilian_aicharacter_2))
  (bind _returnvalue_2 (Transformation|GetActorLocation _as_bp_civilian_aicharacter))
  (bind _returnvalue_3 (Math|Rotator|FindLookatRotation _returnvalue_2 _returnvalue))
  (bind _returnvalue_4 (Math|Vector|GetForwardVector _returnvalue_3))
  (bind _returnvalue_5 (* _returnvalue_4 -5e+02))
  (bind _returnvalue_6 (+ _returnvalue_2 _returnvalue_5))
  (bind (_x _y) (Math|Vector|BreakVector _returnvalue_6))
  (AI|AIMoveTo (Variables|Default|GetAs%20BP%20Civilian%20AICharacter) (Math|Vector|MakeVector _x _y (.Z (Math|Vector|BreakVector _returnvalue_2))) 0 5.0 false
    (:OnSuccess
      (AI|BehaviorTree|FinishExecute true))
    (:OnFail
      (AI|BehaviorTree|FinishExecute false))))

(event EventReceiveExecuteAI
  (params (OwnerController :type AI%20Controller%20Object%20Reference) (ControlledPawn :type Pawn%20Object%20Reference))
  (bind _asbp_civilian_aicharacter (Utilities|Casting|CastToBP_CivilianAICharacter ControlledPawn))
  (Variables|Default|SetAs%20BP%20Civilian%20AICharacter _asbp_civilian_aicharacter)
  (CallFunction|RunAway))