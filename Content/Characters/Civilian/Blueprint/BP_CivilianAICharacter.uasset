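; Civilian NPC AI character that reacts to enemy AI characters and can be talked to.
; On begin play it sets an initial alert state and writes its hide point to the blackboard.
; Seeing an enemy switches the alert state, which a retriggerable delay reverts if the civilian is still alive.
; Interaction stops the AI, focuses it on the interacting character and shows a state-based dialogue message before clearing focus.
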(event OnSeePawn(PawnSensing)
  (params (Pawn :type Pawn%20Object%20Reference))
  (bind _isdead (CallFunction|IsDead))
  (if (not _isdead)
    (Utilities|Casting|CastToBP_EnemyAICharacter Pawn)
    (Utilities|FlowControl|Sequence
      (:then_0
        (CallFunction|UpdateAlertState "NewEnumerator1"))
      (:then_1
        (Utilities|FlowControl|RetriggerableDelay 5.0)
        (bind _isdead_2 (CallFunction|IsDead))
        (if (not _isdead_2)
          (CallFunction|UpdateAlertState "NewEnumerator0"))))))

(event EventInteract
  (params (Character :type BP%20Base%20Character%20Object%20Reference))
  (bind _self self)
  (bind _returnvalue (AI|GetAIController _self))
  (Default|LockMovement Character)
  (AI|Navigation|StopMovement _returnvalue)
  (AI|SetFocus _returnvalue Character)
  (bind _npcdialoguewidget (Variables|Default|GetNPCDialogueWidget)
    (:then
      (Default|InteractMessage _npcdialoguewidget (Variables|Default|GetAI%20State))
      (Variables|Default|SetIsInteracting true)
      (Utilities|FlowControl|RetriggerableDelay 2.0) ; Stop for at least 5 seconds
      (AI|ClearFocus _returnvalue)
      (CallFunction|UnlockMovement)
      (Variables|Default|SetIsInteracting false))
    (:else
      (Development|PrintString "HUH"))))

(event EventBeginPlay
  (|CallParentFunction)
  (CallFunction|UpdateAlertState "NewEnumerator0")
  (AI|Components|Blackboard|SetValueasObject (AI|GetBlackboard (Pawn|GetController)) (Variables|Default|GetHidePointKey) (Variables|Default|GetHidePoint)))

(fn ConstructionScript
  (|CallParentFunction))

(fn GetObjectName
  (return ""))