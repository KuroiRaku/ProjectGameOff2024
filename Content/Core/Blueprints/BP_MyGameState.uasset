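; BP_MyGameState is a game state Blueprint that holds the player list, the level to play and a main menu level reference.
; UpdatePlayerList copies PlayerArray into AllPlayerStates, while UpdateLevelToPlay sets LevelToPlay only with authority and prints a warning otherwise.
; AllPlayerStates and LevelToPlay have empty RepNotify functions, and getters expose both level values.
; BeginPlay only casts the game mode to BP_FirstPersonGameMode, with no further action.
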(event Custom|UpdatePlayerList
  (Variables|Default|SetAllPlayerStates (Variables|Default|GetPlayerArray)))

(event Custom|UpdateLevelToPlay
  (params (LevelToPlay :type World%20Soft%20Object%20Reference))
  (if (Ability|HasAuthority)
    (Variables|Default|SetLevelToPlay LevelToPlay)
    (else
      (Development|PrintString "BRUH, You Not Supposed to Get This Message!"))))

(event EventBeginPlay
  (Utilities|Casting|CastToBP_FirstPersonGameMode (Game|GetGameMode)))

(fn ConstructionScript)

(fn OnRepAllPlayerStates)

(fn OnRepLeveltoPlay)

(fn GetMainMenuLevel
  (return (Variables|Default|GetMainMenuLevel)))

(fn GetLeveltoPlay
  (return (Variables|Default|GetLevelToPlay)))