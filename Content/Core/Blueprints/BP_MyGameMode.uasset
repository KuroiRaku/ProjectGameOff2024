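; BP_MyGameMode is a game mode that handles player respawning at checkpoints and tracks players joining and leaving.
; It caches BP_MyGameState on BeginPlay, then fires join or leave dispatchers on login and logout before asking that state to update its player list.
; RespawnPlayer destroys player 0's character, spawns a new BP_PlayerCharacter at the last checkpoint, or the default transform if none is valid, and possesses it.
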(event Custom|Respawn%20Player
  (Actor|DestroyActor (Game|GetPlayerCharacter 0))
  (bind _lastcheckpoint (Variables|Default|GetLastCheckpoint)
    (:then
      (bind _returnvalue (Game|SpawnActorfromClass "/Game/Core/Blueprints/Character/BP_PlayerCharacter.BP_PlayerCharacter_C" (Math|Transform|MakeTransform (.location (Transformation|GetWorldTransform (Variables|/Game/Core/Blueprints/Checkpoint/BP_Checkpoint.BP_Checkpoint_C|GetPOS _lastcheckpoint))) (.rotation (Transformation|GetWorldTransform (Variables|/Game/Core/Blueprints/Checkpoint/BP_Checkpoint.BP_Checkpoint_C|GetPOS _lastcheckpoint))) "1.000000,1.000000,1.000000") "AlwaysSpawn" "MultiplyWithRoot" 0 "Default Name" "NewEnumerator17" 0))
      (Pawn|Possess (Game|GetPlayerController 0) _returnvalue))
    (:else
      (bind _returnvalue_2 (Game|SpawnActorfromClass "/Game/Core/Blueprints/Character/BP_PlayerCharacter.BP_PlayerCharacter_C" (Math|Transform|MakeTransform "0, 0, 0" "0, 0, 0" "1.000000,1.000000,1.000000") "AlwaysSpawn" "MultiplyWithRoot" 0 "Default Name" "NewEnumerator17" 0))
      (Pawn|Possess (Game|GetPlayerController 0) _returnvalue_2))))

(event EventBeginPlay
  (bind _asbp_my_game_state (Utilities|Casting|CastToBP_MyGameState (Game|GetGameState)))
  (Variables|Default|SetMyGameState _asbp_my_game_state))

(event EventPostLogin
  (params (NewPlayer :type Player%20Controller%20Object%20Reference))
  (Default|CallOnPlayerJoined NewPlayer)
  (Default|UpdatePlayerList (Variables|Default|GetMyGameState)))

(event EventOnLogout
  (params (ExitingController :type Controller%20Object%20Reference))
  (Default|CallOnPlayerLeft ExitingController)
  (Default|UpdatePlayerList (Variables|Default|GetMyGameState)))

(fn ConstructionScript)