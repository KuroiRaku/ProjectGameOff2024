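; BP_Map is a map item that shows a full map widget on screen while it is picked up.
; The construction script creates a BP_MapWidget and sets its image from the Texture variable when that is valid.
; PickUp adds the widget to the viewport and sets IsReading, while PutDown removes it and clears the flag.
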(event EventBeginPlay
  (|CallParentFunction) ; This node is disabled and will not be called.\nDrag off pins to build functionality.
)

(event Collision|EventActorBeginOverlap
  (params (OtherActor :type Actor%20Object%20Reference))
  (|CallParentFunction OtherActor) ; This node is disabled and will not be called.\nDrag off pins to build functionality.
)

(event EventTick
  (params (DeltaSeconds :type Float%20%28single-precision%29))
  (|CallParentFunction DeltaSeconds) ; This node is disabled and will not be called.\nDrag off pins to build functionality.
)

(event EventPutDown
  (Widget|RemovefromParent (Variables|Default|GetMapWidget))
  (Variables|Default|SetIsReading? false))

(event EventPickUp
  (UserInterface|Viewport|AddtoViewport (Variables|Default|GetMapWidget) 0)
  (Variables|Default|SetIsReading? true))

(fn ConstructionScript
  (|CallParentFunction)
  (bind _returnvalue (Game|ConstructObjectfromClass "/Game/UI/BP_MapWidget.BP_MapWidget_C"))
  (bind _output_get (Variables|Default|SetMapWidget _returnvalue))
  (bind _texture (Variables|Default|GetTexture)
    (:then
      (Default|SetImage _output_get _texture))
    (:else)))