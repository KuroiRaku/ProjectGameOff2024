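; BP_HealingCircle is an area pickup that heals BP_BaseCharacter actors entering its HealingArea.
; In one-shot mode it heals the first character to overlap, then destroys itself.
; With PermanentHealingCircle set, it tracks overlapping characters and a looping one-second timer heals each of them until they leave.
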(event OnComponentBeginOverlap(HealingArea)
  (params (OverlappedComponent :type Primitive%20Component%20Object%20Reference) (OtherActor :type Actor%20Object%20Reference) (OtherComp :type Primitive%20Component%20Object%20Reference) (OtherBodyIndex :type Integer) (bFromSweep :type Boolean) (SweepResult :type Hit%20Result%20Structure%20%28by%20ref%29))
  (bind _asbp_base_character (Utilities|Casting|CastToBP_BaseCharacter OtherActor))
  (if (Variables|Default|GetPermanentHealingCircle)
    (Utilities|Array|Add (Variables|Default|GetOverlappedActor) _asbp_base_character)
    (else
      (Default|Heal _asbp_base_character (Variables|Default|GetHealingValue))
      (Actor|DestroyActor))))

(event OnComponentEndOverlap(HealingArea)
  (params (OverlappedComponent :type Primitive%20Component%20Object%20Reference) (OtherActor :type Actor%20Object%20Reference) (OtherComp :type Primitive%20Component%20Object%20Reference) (OtherBodyIndex :type Integer))
  (bind _asbp_base_character (Utilities|Casting|CastToBP_BaseCharacter OtherActor))
  (Utilities|Array|RemoveItem (Variables|Default|GetOverlappedActor) _asbp_base_character))

(event Custom|Healing%20Over%20Time
  (for _array_element (Variables|Default|GetOverlappedActor)
    (Default|Heal _array_element (Variables|Default|GetHealingValue))))

(event EventBeginPlay
  (if (Variables|Default|GetPermanentHealingCircle)
    (Utilities|Time|SetTimerbyEvent (delegate Custom|Healing%20Over%20Time) 1.0 true)))

(fn ConstructionScript)