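; BP_Cage is a destructible cage item that tracks the characters held inside it as hostages.
; On BeginPlay it adds every BP_BaseCharacter overlapping the Cage component to the Hostages array.
; The Damage event subtracts from HealthPoint and destroys the cage at zero or below, with no hostage release logic in this graph.
; A LockMovement call on the characters exists but is disconnected, so it never runs.
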(event EventBeginPlay
  (for _array_element (Collision|GetOverlappingActors (Variables|Default|GetCage) "/Game/Core/Blueprints/Character/BP_BaseCharacter.BP_BaseCharacter_C" :!class /Script/Engine.PrimitiveComponent)
    (bind _asbp_base_character (Utilities|Casting|CastToBP_BaseCharacter _array_element))
    (Utilities|Array|Add (Variables|Default|GetHostages) _asbp_base_character)))

(event EventDamage
  (params (Damage :type Float%20%28double-precision%29))
  (bind _output_get (Variables|Default|SetHealthPoint (- (Variables|Default|GetHealthPoint) Damage)))
  (if (<= _output_get 0.0)
    (Actor|DestroyActor)))

(fn ConstructionScript)