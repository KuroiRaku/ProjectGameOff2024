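; Character component that manages four spell slots, each built from an element, shape, size and speed combination.
; It loads property data tables and per-unit progression, then sums the four parts' stats per slot and takes visuals and sounds from an element-plus-shape resource row.
; ShootProjectile checks cooldown and mana, then spawns BP_SpellObject with those properties.
; Teach events unlock types and slots, and debug keys print the state.
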(event Custom|Teach%20Speed%20Type
  (params (Speed%20Type :type EMagicSpeed%20Enum :default "Fast"))
  ;[1 1 1] Progression Unlock
  (Utilities|Map|Add (Variables|Default|GetSpeedTypeProgressionMap) Speed%20Type true))

(event Custom|Teach%20Element%20Type
  (params (Element%20Type :type EMagicElement%20Enum :default "Water"))
  ;[1 1 1] Progression Unlock
  (Utilities|Map|Add (Variables|Default|GetElementTypeProgressionMap) Element%20Type true))

(event Custom|Print%20Magic%20Info
  (bind _selectedspellslot (Variables|Default|GetSelectedSpellSlot))
  (bind _spellinfomap (Variables|Default|GetSpellInfoMap))
  (bind (_value _returnvalue) (Utilities|Map|Find _spellinfomap _selectedspellslot))
  (bind (_element _shape _size _speed) (Utilities|Struct|BreakMagicInfo _value))
  ;[0.4055 0.8325 1] Debug Print
  ;;[1 1 1] Print Current Selected Slot
  (if _returnvalue
    (Development|PrintString (Utilities|String|Append "Element: " (Utilities|String|EnumtoString _element) " 
Shape" (Utilities|String|EnumtoString _shape) " 
Size: " (Utilities|String|EnumtoString _size) " 
Speed:" (Utilities|String|EnumtoString _speed)))))

(event Custom|Print%20Progression
  ;[0.4055 0.8325 1] Debug Print
  ;;[1 1 1] Print Progresion
  (bind _enumvalue (|ForEachEMagicElement)
    (:LoopBody
      (Development|PrintString (Utilities|String|Append (Utilities|String|EnumtoString _enumvalue) "  " (Utilities|String|ToString(Boolean) (.Value (Utilities|Map|Find (Variables|Default|GetElementTypeProgressionMap) _enumvalue))))))
    (:then
      (bind _enumvalue_2 (|ForEachEMagicSpeed)
        (:LoopBody
          (Development|PrintString (Utilities|String|Append (Utilities|String|EnumtoString _enumvalue_2) "  " (Utilities|String|ToString(Boolean) (.Value (Utilities|Map|Find (Variables|Default|GetSpeedTypeProgressionMap) _enumvalue_2))))))
        (:then
          (bind _enumvalue_3 (|ForEachEMagicShape)
            (:LoopBody
              (Development|PrintString (Utilities|String|Append (Utilities|String|EnumtoString _enumvalue_3) "  " (Utilities|String|ToString(Boolean) (.Value (Utilities|Map|Find (Variables|Default|GetShapeTypeProgression) _enumvalue_3))))))
            (:then
              (bind _enumvalue_4 (|ForEachEMagicSize)
                (:LoopBody
                  (Development|PrintString (Utilities|String|Append (Utilities|String|EnumtoString _enumvalue_4) "  " (Utilities|String|ToString(Boolean) (.Value (Utilities|Map|Find (Variables|Default|GetSizeTypeProgression) _enumvalue_4))))))
                (:then
                  (bind _enumvalue_5 (|ForEachSpellSlotEnum)
                    (:LoopBody
                      (Development|PrintString (Utilities|String|Append (Utilities|String|EnumtoString _enumvalue_5) "  " (Utilities|String|ToString(Boolean) (.Value (Utilities|Map|Find (Variables|Default|GetSpellSlotProgression) _enumvalue_5))))))))))))))))

(event Custom|Print%20Elemenet%20Property
  ;[0.4055 0.8325 1] Debug Print
  (bind _enumvalue (|ForEachEMagicElement)
    (:LoopBody
      (Development|PrintString (Utilities|String|Append "Element: " (Utilities|String|EnumtoString (.ElementType (Utilities|Struct|BreakSpellElementPropertyData (.Value (Utilities|Map|Find (Variables|Default|GetElementPropertyDataMap) _enumvalue))))) " 
Speed" (Utilities|String|ToString(Float) (.Speed (Utilities|Struct|BreakSpellElementPropertyData (.Value (Utilities|Map|Find (Variables|Default|GetElementPropertyDataMap) _enumvalue))))) " 
Damage: " (Utilities|String|ToString(Float) (.Damage (Utilities|Struct|BreakSpellElementPropertyData (.Value (Utilities|Map|Find (Variables|Default|GetElementPropertyDataMap) _enumvalue))))) " 
Cooldown Time: " (Utilities|String|ToString(Float) (.CooldownTime (Utilities|Struct|BreakSpellElementPropertyData (.Value (Utilities|Map|Find (Variables|Default|GetElementPropertyDataMap) _enumvalue))))) " 
Time Before dissipating" (Utilities|String|ToString(Float) (.TimeBeforeDissipating (Utilities|Struct|BreakSpellElementPropertyData (.Value (Utilities|Map|Find (Variables|Default|GetElementPropertyDataMap) _enumvalue))))) " 
Mana Cost: " (Utilities|String|ToString(Float) (.ManaCost (Utilities|Struct|BreakSpellElementPropertyData (.Value (Utilities|Map|Find (Variables|Default|GetElementPropertyDataMap) _enumvalue))))) " 
Hitpoint" (Utilities|String|ToString(Float) (.Hitpoint (Utilities|Struct|BreakSpellElementPropertyData (.Value (Utilities|Map|Find (Variables|Default|GetElementPropertyDataMap) _enumvalue))))))))))

(event Custom|SelectSpellSlot1
  ;[1 1 1] Select Spell Slot
  (Variables|Default|SetSelectedSpellSlot "NewEnumerator0")
  (CallFunction|PrintMagicInfo))

(event Custom|SelectSpellSlot2
  ;[1 1 1] Select Spell Slot
  (if (.Value (Utilities|Map|Find (Variables|Default|GetSpellSlotProgression) "NewEnumerator1"))
    (Variables|Default|SetSelectedSpellSlot "NewEnumerator1")
    (CallFunction|PrintMagicInfo)))

(event Custom|SelectSpellSlot3
  ;[1 1 1] Select Spell Slot
  (if (.Value (Utilities|Map|Find (Variables|Default|GetSpellSlotProgression) "NewEnumerator2"))
    (Variables|Default|SetSelectedSpellSlot "NewEnumerator2")
    (CallFunction|PrintMagicInfo)))

(event Custom|SelectSpellSlot4
  ;[1 1 1] Select Spell Slot
  (if (.Value (Utilities|Map|Find (Variables|Default|GetSpellSlotProgression) "NewEnumerator3"))
    (Variables|Default|SetSelectedSpellSlot "NewEnumerator3")
    (CallFunction|PrintMagicInfo)))

(event Custom|UnlockAllSpells
  (bind _enumvalue (|ForEachSpellSlotEnum)
    (:LoopBody
      (Utilities|Map|Add (Variables|Default|GetSpellSlotProgression) _enumvalue true))
    (:then
      (bind _enumvalue_2 (|ForEachEMagicElement)
        (:LoopBody
          (Utilities|Map|Add (Variables|Default|GetElementTypeProgressionMap) _enumvalue_2 false))
        (:then
          (bind _enumvalue_3 (|ForEachEMagicSpeed)
            (:LoopBody
              (Utilities|Map|Add (Variables|Default|GetSpeedTypeProgressionMap) _enumvalue_3 true))
            (:then
              (bind _enumvalue_4 (|ForEachEMagicSize)
                (:LoopBody
                  (Utilities|Map|Add (Variables|Default|GetSizeTypeProgression) _enumvalue_4 false))
                (:then
                  (bind _enumvalue_5 (|ForEachEMagicShape)
                    (:LoopBody
                      (Utilities|Map|Add (Variables|Default|GetShapeTypeProgression) _enumvalue_5 false))))))))))))

(event Custom|Shoot%20Projectile
  (params (ProjectileSpawnTransform :type Transform))
  (bind _returnvalue (Utilities|Time|GetGameTimeinSeconds))
  (bind _selectedspellslot (Variables|Default|GetSelectedSpellSlot))
  (bind _spellpropertymap (Variables|Default|GetSpellPropertyMap))
  (bind _selectedspellslot_2 (Variables|Default|GetSelectedSpellSlot))
  (bind _spellslotcooldownfloat (Variables|Default|GetSpellSlotCoolDownFloat))
  (bind (_value _returnvalue_2) (Utilities|Map|Find _spellpropertymap _selectedspellslot))
  (bind _value_2 (Utilities|Map|Find _spellslotcooldownfloat _selectedspellslot))
  (bind (_spellmaterial _spellmesh _meshrotation _meshrelativelocation _meshrelativescale _shootingsoundeffect _chargingupsoundeffect _impactsoundeffect _spellvfx _spellvanishingvfx _spellicon _hitpoint _speed _timebeforedissipating _damage _charginguptime _scale _manacost _cooldowntime _accuracy _spellelement) (Utilities|Struct|BreakSpellProperty _value))
  ;[1 1 1 1 44] Shooting Projectiles
  (Math|Float|CompareFloat _value_2 _returnvalue
    (:>
      (Development|PrintString (Utilities|String|Append (Utilities|String|EnumtoString _selectedspellslot) " On Cooldown" (Utilities|String|ToString(Float) (- _value_2 _returnvalue)))))
    (:<
      (if _returnvalue_2
        (bind _hasmana (CallFunction|CheckManaCondition))
        (if _hasmana
          (Game|SpawnActorfromClass "/Game/Core/Blueprints/MagicComponent/BP_SpellObject.BP_SpellObject_C" ProjectileSpawnTransform "Undefined" "MultiplyWithRoot" 0 _hitpoint _damage _timebeforedissipating _spellelement _speed (Variables|Default|GetCharacter) _spellvfx _spellvanishingvfx _spellmesh _spellmaterial _scale _impactsoundeffect _meshrotation _meshrelativelocation _meshrelativescale 0)
          (Audio|SpawnSoundatLocation _shootingsoundeffect (.Location (Math|Transform|BreakTransform ProjectileSpawnTransform)) "0, 0, 0" 1.0 1.0 0.0 0 0)
          (Utilities|Map|Add (Variables|Default|GetSpellSlotCoolDownFloat) _selectedspellslot_2 (+ _cooldowntime (Utilities|Time|GetGameTimeinSeconds))) ; Cooldown!!!
          (Default|CallCooldownEventDispatcher _cooldowntime _selectedspellslot_2) ; Allow UI to get the maximum value of cooldown
          (elif (Variables|/Game/Core/Blueprints/Character/BP_BaseCharacter.BP_BaseCharacter_C|GetIsPlayer (Variables|Default|GetCharacter))
            (Audio|PlaySound2D "/Game/Assets/SFX/UI-SFX/OutOfMana/OUT_OF_MANA_SFX.OUT_OF_MANA_SFX" 1.0 1.0 0.0 0 0)
            (Development|PrintString "Not Enough Mana")))
        (else
          (Development|PrintString "Spell Property Not Found... while shooting"))))))

(event Custom|Teach%20Shape%20Type
  (params (Shape%20Type :type EMagicShape%20Enum :default "Arrow"))
  ;[1 1 1] Progression Unlock
  (Utilities|Map|Add (Variables|Default|GetShapeTypeProgression) Shape%20Type true))

(event Custom|Teach%20Size%20Type
  (params (Size%20Type :type EMagicSize%20Enum :default "Small"))
  ;[1 1 1] Progression Unlock
  (Utilities|Map|Add (Variables|Default|GetSizeTypeProgression) Size%20Type true))

(event Custom|BuildSpell
  (params (Spell%20Slot :type SpellSlotEnum%20Enum :default "NewEnumerator0"))
  ;[1 1 1] When Spell Info is changed (on UI) UI Will directly modify SpellInfoMap
  (CallFunction|ProcessSpellInfo Spell%20Slot))

(event Custom|Teach%20Magic%20Slot
  (params (Slot :type SpellSlotEnum%20Enum :default "NewEnumerator0"))
  ;[1 1 1] Progression Unlock
  (Utilities|Map|Add (Variables|Default|GetSpellSlotProgression) Slot true))

(event Custom|LoadFromDataTable
  ;[1 1 1] Read from Data Tables, should be done in Constructor nodes in Base_Characters
  ; Load Magic Properties
  (bind _enumvalue (|ForEachEMagicElement)
    (:LoopBody
      (bind _returnvalue (Utilities|GetDataTableRow "/Game/Core/Blueprints/MagicComponent/SpellElementPropertyDataTable.SpellElementPropertyDataTable" (Utilities|String|StringToName (Utilities|String|EnumtoString _enumvalue)))
        (:then
          (Utilities|Map|Add (Variables|Default|GetElementPropertyDataMap) _enumvalue _returnvalue))
        (:RowNotFound
          (Development|PrintString (Utilities|String|Append (Utilities|String|EnumtoString _enumvalue) " NOT FOUND IN DATA TABLE")))))
    (:then
      (bind _enumvalue_2 (|ForEachEMagicShape)
        (:LoopBody
          (bind _returnvalue_2 (Utilities|GetDataTableRow "/Game/Core/Blueprints/MagicComponent/SpellShapePropertyDataTable.SpellShapePropertyDataTable" (Utilities|String|StringToName (Utilities|String|EnumtoString _enumvalue_2)))
            (:then
              (Utilities|Map|Add (Variables|Default|GetShapePropertyDataMap) _enumvalue_2 _returnvalue_2))
            (:RowNotFound
              (Development|PrintString (Utilities|String|Append (Utilities|String|EnumtoString _enumvalue_2) " NOT FOUND IN DATA TABLE")))))
        (:then
          (bind _enumvalue_3 (|ForEachEMagicSize)
            (:LoopBody
              (bind _returnvalue_3 (Utilities|GetDataTableRow "/Game/Core/Blueprints/MagicComponent/SpellSizeDataTable.SpellSizeDataTable" (Utilities|String|StringToName (Utilities|String|EnumtoString _enumvalue_3)))
                (:then
                  (Utilities|Map|Add (Variables|Default|GetSizePropertyDataMap) _enumvalue_3 _returnvalue_3))
                (:RowNotFound
                  (Development|PrintString (Utilities|String|Append (Utilities|String|EnumtoString _enumvalue_3) " NOT FOUND IN DATA TABLE")))))
            (:then
              (bind _enumvalue_4 (|ForEachEMagicSpeed)
                (:LoopBody
                  (bind _returnvalue_4 (Utilities|GetDataTableRow "/Game/Core/Blueprints/MagicComponent/SpellSpeedTypePropertyDataTable.SpellSpeedTypePropertyDataTable" (Utilities|String|StringToName (Utilities|String|EnumtoString _enumvalue_4)))
                    (:then
                      (Utilities|Map|Add (Variables|Default|GetSpeedPropertyDataMap) _enumvalue_4 _returnvalue_4))
                    (:RowNotFound
                      (Development|PrintString (Utilities|String|Append (Utilities|String|EnumtoString _enumvalue_4) " NOT FOUND IN DATA TABLE")))))
                (:then
                  (bind _asbp_base_character (Utilities|Casting|CastToBP_BaseCharacter (Components|GetOwner))
                    (:then
                      (Variables|Default|SetCharacter _asbp_base_character)
                      (if true
                        (CallFunction|LoadUnitProgression)))
                    (:CastFailed
                      (Development|PrintString "Unable to Cast Owner to BP Base Character")))
                  (CallFunction|ProcessSpellInfo "NewEnumerator0")
                  (CallFunction|ProcessSpellInfo "NewEnumerator1")
                  (CallFunction|ProcessSpellInfo "NewEnumerator2")
                  (CallFunction|ProcessSpellInfo "NewEnumerator3"))))))))))

(event Custom|Print%20Magic%20Properties
  (bind _spellpropertymap (Variables|Default|GetSpellPropertyMap))
  (bind _selectedspellslot (Variables|Default|GetSelectedSpellSlot))
  (bind (_value _returnvalue) (Utilities|Map|Find _spellpropertymap _selectedspellslot))
  (bind (_spellmaterial _spellmesh _meshrotation _meshrelativelocation _meshrelativescale _shootingsoundeffect _chargingupsoundeffect _impactsoundeffect _spellvfx _spellvanishingvfx _spellicon _hitpoint _speed _timebeforedissipating _damage _charginguptime _scale _manacost _cooldowntime _accuracy _spellelement) (Utilities|Struct|BreakSpellProperty _value))
  ;[0.4055 0.8325 1] Debug Print
  ;;[1 1 1] Print Spell PRoperty
  (if _returnvalue
    (Development|PrintString (Utilities|String|Append "Element: " (Utilities|String|EnumtoString _spellelement) " 
Mesh: " (Utilities|GetDisplayName _spellmesh) " 
Material " (Utilities|GetDisplayName _spellmaterial) " 
Sound Effect: " (Utilities|GetDisplayName _shootingsoundeffect) " 
Spell VFX: " (Utilities|GetDisplayName _spellvfx) " 
Spell Icon: " (Utilities|GetDisplayName _spellicon) " 
Speed" (Utilities|String|ToString(Float) _speed) " 
Damage: " (Utilities|String|ToString(Float) _damage) " 
Cooldown Time: " (Utilities|String|ToString(Float) _cooldowntime) " 
Time Before dissipating" (Utilities|String|ToString(Float) _timebeforedissipating) " 
Mana Cost: " (Utilities|String|ToString(Float) _manacost)))))

(event Custom|Load%20Unit%20Progression
  (bind _character (Variables|Default|GetCharacter))
  (bind _character_type (Variables|/Game/Core/Blueprints/Character/BP_BaseCharacter.BP_BaseCharacter_C|GetCharacter%20Type _character))
  (bind _returnvalue (Utilities|String|EnumtoString _character_type))
  ;[1 1 1] Load Progression
  (bind _returnvalue_2 (Utilities|GetDataTableRow "/Game/Core/Blueprints/Character/UnitInfoDataTable.UnitInfoDataTable" (Utilities|String|StringToName _returnvalue))
    (:then
      (Variables|Default|SetSizeTypeProgression (.SizeTypeEnabledMap (Utilities|Struct|BreakUnitInfo _returnvalue_2)))
      (Variables|Default|SetSpellSlotProgression (.SpellSlotEnabledMap (Utilities|Struct|BreakUnitInfo _returnvalue_2)))
      (Variables|Default|SetSpellInfoMap (.SpellInfoMap (Utilities|Struct|BreakUnitInfo _returnvalue_2)))
      (Variables|Default|SetSpeedTypeProgressionMap (.SpeedTypeEnabledMap (Utilities|Struct|BreakUnitInfo _returnvalue_2)))
      (Variables|Default|SetShapeTypeProgression (.ShapeTypeEnabledMap (Utilities|Struct|BreakUnitInfo _returnvalue_2)))
      (Variables|Default|SetElementTypeProgressionMap (.ElementTypeEnabledMap (Utilities|Struct|BreakUnitInfo _returnvalue_2))))
    (:RowNotFound
      (Development|PrintString (Utilities|String|Append _returnvalue " Unit Type Not Found, Please Create One")))))

(event Input|KeyboardEvents|M
  (params (Key :type Key%20Structure))
  (:Pressed
    (CallFunction|PrintProgression)))

(event Input|KeyboardEvents|N
  (params (Key :type Key%20Structure))
  (:Pressed
    (CallFunction|PrintMagicProperties)))

(event Input|KeyboardEvents|B
  (params (Key :type Key%20Structure))
  (:Pressed
    (CallFunction|PrintElemenetProperty)))

(fn ProcessSpellInfo
  (params (SpellSlot :type SpellSlotEnum%20Enum :default "NewEnumerator0"))
  (bind _shapepropertydatamap (Variables|Default|GetShapePropertyDataMap))
  (bind _spellpropertymap (Variables|Default|GetSpellPropertyMap))
  (bind _elementpropertydatamap (Variables|Default|GetElementPropertyDataMap))
  (bind _spellinfomap (Variables|Default|GetSpellInfoMap))
  (bind _speedpropertydatamap (Variables|Default|GetSpeedPropertyDataMap))
  (bind _sizepropertydatamap (Variables|Default|GetSizePropertyDataMap))
  (bind _value (Utilities|Map|Find _spellinfomap SpellSlot))
  (bind (_element _shape _size _speed) (Utilities|Struct|BreakMagicInfo _value))
  (bind _value_2 (Utilities|Map|Find _elementpropertydatamap _element))
  (bind _value_3 (Utilities|Map|Find _speedpropertydatamap _speed))
  (bind _value_4 (Utilities|Map|Find _sizepropertydatamap _size))
  (bind _value_5 (Utilities|Map|Find _shapepropertydatamap _shape))
  (bind _returnvalue (Utilities|String|EnumtoString _element))
  (bind _returnvalue_2 (Utilities|String|EnumtoString _shape))
  (bind (_elementtype _damage _speed_2 _manacost _charginguptime _accuracy _timebeforedissipating _hitpoint _cooldowntime) (Utilities|Struct|BreakSpellElementPropertyData _value_2))
  (bind (_shapetype _damage_2 _speed_3 _manacost_2 _charginguptime_2 _accuracy_2 _timebeforedissipating_2 _hitpoint_2 _cooldowntime_2) (Utilities|Struct|BreakSpellShapePropertyData _value_5))
  (bind (_sizetype _damage_3 _speed_4 _manacost_3 _charginguptime_3 _accuracy_3 _timebeforedissipating_3 _hitpoint_3 _cooldowntime_3 _scalemultiplier) (Utilities|Struct|BreakSpellSizePropertyData _value_4))
  (bind (_speedtype _damage_4 _speed_5 _manacost_4 _charginguptime_4 _accuracy_4 _timebeforedissipating_4 _hitpoint_4 _cooldowntime_4) (Utilities|Struct|BreakSpellSpeedPropertyData _value_3))
  (bind _returnvalue_3 (Utilities|String|Append _returnvalue _returnvalue_2))
  (bind _returnvalue_4 (+ _cooldowntime _cooldowntime_2 _cooldowntime_3 _cooldowntime_4))
  (bind _returnvalue_5 (+ _manacost _manacost_2 _manacost_3 _manacost_4))
  (bind _returnvalue_6 (+ _damage _damage_2 _damage_3 _damage_4))
  (bind _returnvalue_7 (+ _charginguptime _charginguptime_2 _charginguptime_3 _charginguptime_4))
  (bind _returnvalue_8 (+ _accuracy _accuracy_2 _accuracy_3 _accuracy_4))
  (bind _returnvalue_9 (+ _timebeforedissipating _timebeforedissipating_2 _timebeforedissipating_3 _timebeforedissipating_4))
  (bind _returnvalue_10 (+ _hitpoint _hitpoint_2 _hitpoint_3 _hitpoint_4))
  (bind _returnvalue_11 (Utilities|GetDataTableRow "/Game/Core/Blueprints/MagicComponent/SpellResourceDataTable.SpellResourceDataTable" (Utilities|String|StringToName _returnvalue_3))
    (:then
      (if (Utilities|Enum|Equal(Enum) _speed "Stationary")
        (Utilities|Map|Add _spellpropertymap SpellSlot (Utilities|Struct|MakeSpellProperty (.SpellElementMaterial (Utilities|Struct|BreakSpellResourceData _returnvalue_11)) (.SpellShapeStaticMesh (Utilities|Struct|BreakSpellResourceData _returnvalue_11)) (.Rotation (Utilities|Struct|BreakSpellResourceData _returnvalue_11)) (.Location (Utilities|Struct|BreakSpellResourceData _returnvalue_11)) (.Scale (Utilities|Struct|BreakSpellResourceData _returnvalue_11)) (.ShootingSoundEffect (Utilities|Struct|BreakSpellResourceData _returnvalue_11)) (.ChargingUpSoundEffect (Utilities|Struct|BreakSpellResourceData _returnvalue_11)) 0 (.VFXFile (Utilities|Struct|BreakSpellResourceData _returnvalue_11)) (.VanishVFX (Utilities|Struct|BreakSpellResourceData _returnvalue_11)) (.SpellIcon (Utilities|Struct|BreakSpellResourceData _returnvalue_11)) _returnvalue_10 0.0 _returnvalue_9 _returnvalue_6 _returnvalue_7 _scalemultiplier _returnvalue_5 _returnvalue_4 _returnvalue_8 _element))
        (else
          (Utilities|Map|Add _spellpropertymap SpellSlot (Utilities|Struct|MakeSpellProperty (.SpellElementMaterial (Utilities|Struct|BreakSpellResourceData _returnvalue_11)) (.SpellShapeStaticMesh (Utilities|Struct|BreakSpellResourceData _returnvalue_11)) (.Rotation (Utilities|Struct|BreakSpellResourceData _returnvalue_11)) (.Location (Utilities|Struct|BreakSpellResourceData _returnvalue_11)) (.Scale (Utilities|Struct|BreakSpellResourceData _returnvalue_11)) (.ShootingSoundEffect (Utilities|Struct|BreakSpellResourceData _returnvalue_11)) (.ChargingUpSoundEffect (Utilities|Struct|BreakSpellResourceData _returnvalue_11)) (.ImpactSound (Utilities|Struct|BreakSpellResourceData _returnvalue_11)) (.VFXFile (Utilities|Struct|BreakSpellResourceData _returnvalue_11)) (.VanishVFX (Utilities|Struct|BreakSpellResourceData _returnvalue_11)) (.SpellIcon (Utilities|Struct|BreakSpellResourceData _returnvalue_11)) _returnvalue_10 (+ _speed_2 _speed_3 _speed_4 _speed_5) _returnvalue_9 _returnvalue_6 _returnvalue_7 _scalemultiplier _returnvalue_5 _returnvalue_4 _returnvalue_8 _element)))))
    (:RowNotFound
      (Development|PrintString (Utilities|String|Append _returnvalue_3 " NOT FOUND IN DATA TABLE") true true "(R=0.000000,G=0.660000,B=1.000000,A=1.000000)" 5.0)
      (Utilities|Map|Add _spellpropertymap SpellSlot (Utilities|Struct|MakeSpellProperty "/Game/Core/Blueprints/PlayerMeshtem/Alpha_Body_MAT.Alpha_Body_MAT" "/Engine/EditorMeshes/EditorSphere.EditorSphere" "0.000000,0.000000,0.000000" "0.000000,0.000000,0.000000" "1.000000,1.000000,1.000000" "/Engine/EditorSounds/GamePreview/StartSimulate_Cue.StartSimulate_Cue" "/Engine/VREditor/Sounds/UI/Click_on_Button_Cue.Click_on_Button_Cue" 0 "/Game/Assets/Cursor/FX_Cursor.FX_Cursor" 0 "/Engine/Tutorial/Mobile/TutorialAssets/android_Icon.android_Icon" 1e+02 4.0 5.0 1e+02 2.0 1.0 1.0 1.0 1.0 "Water"))))
  (return))

(fn GetCurrentSelectedSpellProperty
  (return (.Value (Utilities|Map|Find (Variables|Default|GetSpellPropertyMap) (Variables|Default|GetSelectedSpellSlot)))))

(fn CheckManaCondition
  (bind _character (Variables|Default|GetCharacter))
  (bind _spell_property (CallFunction|GetCurrentSelectedSpellProperty))
  (if (>= (Variables|/Game/Core/Blueprints/Character/BP_BaseCharacter.BP_BaseCharacter_C|GetCurrentMana (Variables|Default|GetCharacter)) (.ManaCost (Utilities|Struct|BreakSpellProperty _spell_property)))
    (if (not (Variables|/Game/Core/Blueprints/Character/BP_BaseCharacter.BP_BaseCharacter_C|GetIsEnemy (Variables|Default|GetCharacter)))
      (Variables|/Game/Core/Blueprints/Character/BP_BaseCharacter.BP_BaseCharacter_C|SetCurrentMana _character (- (Variables|/Game/Core/Blueprints/Character/BP_BaseCharacter.BP_BaseCharacter_C|GetCurrentMana (Variables|Default|GetCharacter)) (.ManaCost (Utilities|Struct|BreakSpellProperty _spell_property))))
      (Default|UpdateMana (Variables|/Game/Core/Blueprints/Character/BP_BaseCharacter.BP_BaseCharacter_C|GetNPCOverheadWidget _character))
      (return true))
    (else
      (Development|PrintString "Not Enough Mana")
      (return false))))