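; Elemental spell actor, configured at construction as a moving projectile or, at zero Speed, a stationary area or solid Earth wall.
; Overlaps damage characters and destroyables, sparing the caster during a short buffer.
; Stationary Fire and Electric damage overlapping characters on a looping timer, while stationary Water heals them.
; Colliding spells resolve by Hitpoint and Damage, and spells expire after a dissipation delay or on impact with sound and VFX.
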(event OnComponentBeginOverlap(SpellObjectMesh)
  (params (OverlappedComponent :type Primitive%20Component%20Object%20Reference) (OtherActor :type Actor%20Object%20Reference) (OtherComp :type Primitive%20Component%20Object%20Reference) (OtherBodyIndex :type Integer) (bFromSweep :type Boolean) (SweepResult :type Hit%20Result%20Structure%20%28by%20ref%29))
  (bind _element (Variables|Default|GetElement))
  ;[1 1 1] Damage Handling On Overlapped
  (Utilities|Casting|CastToWidgetComponent OtherComp ; Please Ignore Widget Component
    (:CastFailed
      (Utilities|Casting|CastToSphereComponent OtherComp
        (:CastFailed
          (if (or (!= OtherActor (Variables|Default|GetSpellCaster)) (>= (Actor|GetGameTimeSinceCreation) (Variables|Default|GetSpellDamageBuffer)))
            (bind _asbp_base_character (Utilities|Casting|CastToBP_BaseCharacter OtherActor)
              (:then
                (if (and (<= (Variables|/Script/Engine.ProjectileMovementComponent|GetInitialSpeed (Variables|Default|GetProjectileMovement)) 0.0) (Utilities|Enum|Equal(Enum) (Variables|Default|GetElement) "Water"))
                  (Variables|Default|SetIsHealing true)
                  (Utilities|Array|Add (Variables|Default|GetOverlappedActors) _asbp_base_character :!label _label)
                  (else
                    (Default|TakeDamage _asbp_base_character (Variables|Default|GetDamage) (Variables|Default|GetStartingLocation))
                    (if (and (<= (Variables|/Script/Engine.ProjectileMovementComponent|GetInitialSpeed (Variables|Default|GetProjectileMovement)) 0.0) (or (Utilities|Enum|Equal(Enum) _element "Fire") (Utilities|Enum|Equal(Enum) _element "Electric")))
                      (goto _label)
                      (else
                        (CallFunction|DestroySelf))))))
              (:CastFailed
                (bind _asbp_spell_object (Utilities|Casting|CastToBP_SpellObject OtherActor)
                  (:then
                    (CallFunction|ProjectileTakeDamage _asbp_spell_object (Variables|Default|GetDamage) (Variables|Default|GetHitpoint) self))
                  (:CastFailed
                    (Utilities|Casting|CastToBP_RTSCameraPawn OtherActor
                      (:CastFailed
                        (bind _asdestroyable (Utilities|Casting|CastToDestroyable OtherActor)
                          (:then
                            (Default|Damage _asdestroyable (Variables|Default|GetDamage))
                            (CallFunction|DestroySelf :!label _label_2))
                          (:CastFailed
                            (Development|PrintString (Utilities|String|Append (Variables|Default|GetWrongObjectDebugString) (Utilities|GetDisplayName OtherComp)))
                            (if (> (Variables|/Script/Engine.ProjectileMovementComponent|GetInitialSpeed (Variables|Default|GetProjectileMovement)) 0.0)
                              (goto _label_2))))))))))))))))

(event OnComponentEndOverlap(SpellObjectMesh)
  (params (OverlappedComponent :type Primitive%20Component%20Object%20Reference) (OtherActor :type Actor%20Object%20Reference) (OtherComp :type Primitive%20Component%20Object%20Reference) (OtherBodyIndex :type Integer))
  ;[1 1 1] Damage Handling On Overlapped
  (bind _asbp_base_character (Utilities|Casting|CastToBP_BaseCharacter OtherActor))
  (Utilities|Array|RemoveItem (Variables|Default|GetOverlappedActors) _asbp_base_character))

(event OnComponentHit(SpellObjectMesh)
  (params (HitComponent :type Primitive%20Component%20Object%20Reference) (OtherActor :type Actor%20Object%20Reference) (OtherComp :type Primitive%20Component%20Object%20Reference) (NormalImpulse :type Vector :default "0, 0, 0") (Hit :type Hit%20Result%20Structure%20%28by%20ref%29))
  ;[1 1 1] For Earth Element, since is gonna be solid
  (bind _asbp_base_character (Utilities|Casting|CastToBP_BaseCharacter OtherActor))
  (if (> (Variables|/Script/Engine.ProjectileMovementComponent|GetInitialSpeed (Variables|Default|GetProjectileMovement)) 0.0)
    (Default|TakeDamage _asbp_base_character (Variables|Default|GetDamage) "0, 0, 0")))

(event Custom|Projectile%20Take%20Damage
  (params (Damage :type Float%20%28double-precision%29) (DamageDealerHitpoint :type Float%20%28double-precision%29) (Other%20Spell%20Projectile :type BP%20Spell%20Object%20Object%20Reference%20%28by%20ref%29))
  (bind _speed (Variables|Default|GetSpeed))
  (bind _speed_2 (Variables|BP_SpellObject_C|GetSpeed Other%20Spell%20Projectile))
  (bind _returnvalue (> _speed_2 0.0))
  (bind _returnvalue_2 (<= _speed 0.0))
  (bind _returnvalue_3 (and _returnvalue _returnvalue_2))
  ;[1 1 1] Deal Damage To Projectiles and Player
  (if (and (== (Variables|BP_SpellObject_C|GetHitpoint Other%20Spell%20Projectile) (Variables|Default|GetHitpoint)) (== (Variables|BP_SpellObject_C|GetDamage Other%20Spell%20Projectile) (Variables|Default|GetDamage)))
    (CallFunction|DestroySelf Other%20Spell%20Projectile)
    (CallFunction|DestroySelf)
    (else
      (bind _output_get (Variables|Default|SetHitpoint (- (Variables|Default|GetHitpoint) Damage)))
      (if (> _output_get 0.0)
        (if (> _output_get DamageDealerHitpoint)
          (Development|PrintString (Utilities|String|Append (Variables|Default|GetSurvivedHitDebugString) (Utilities|String|ToString(Float) _output_get)))
          (else
            (if _returnvalue_3
              (CallFunction|DestroySelf Other%20Spell%20Projectile) ; Destroy other
            )
            (CallFunction|DestroySelf)))
        (else
          (if _returnvalue_3
            (CallFunction|DestroySelf Other%20Spell%20Projectile) ; Destroy other
          )
          (CallFunction|DestroySelf))))))

(event Custom|Destroy%20Self
  (bind _returnvalue (Transformation|GetActorTransform))
  ;[1 1 1] Maybe We Can Spawn VFX upon destruction
  (Audio|SpawnSoundatLocation (Variables|Default|GetImpactSound) (Transformation|GetActorLocation) "0, 0, 0" 1.0 1.0 0.0 0 0)
  (Niagara|SpawnSystematLocation (Variables|Default|GetSpellDistinguishingVFX) (.location _returnvalue) (.rotation _returnvalue) (.scale _returnvalue))
  (Actor|DestroyActor))

(event Custom|Launch
  (params (Direction :type Vector))
  (bind _speed (Variables|Default|GetSpeed))
  ;[1 1 1] Launch the projectile!!!!
  (if (> _speed 0.0)
    (Variables|/Script/Engine.MovementComponent|SetVelocity (Variables|Default|GetProjectileMovement) (+ Direction (* Direction _speed)))))

(event Custom|Damage%20Over%20Time
  (for _array_element (Variables|Default|GetOverlappedActors)
    (if (not (Variables|Default|GetIsHealing))
      (Default|TakeDamage _array_element (Variables|Default|GetDamage) (Variables|Default|GetStartingLocation))
      (else
        (Default|Heal _array_element 2e+01)))))

(event EventBeginPlay
  (bind _element (Variables|Default|GetElement))
  ;[1 1 1] Start Damage Over Time For suitable Element
  (if (and (Math|Boolean|ORBoolean (Utilities|Enum|Equal(Enum) _element "Fire") (Utilities|Enum|Equal(Enum) _element "Electric") (Utilities|Enum|Equal(Enum) _element "Water")) (<= (Variables|Default|GetSpeed) 0.0))
    (Utilities|Time|SetTimerbyEvent (delegate Custom|Damage%20Over%20Time) (Variables|Default|GetInterval) true))
  ;[1 1 1] Destroy itseslf depending on the Time Before Dissipating
  (Utilities|FlowControl|Delay (Variables|Default|GetTimeBeforeDissipating))
  (CallFunction|DestroySelf))

(fn ConstructionScript
  (bind _spellobjectmesh (Variables|Default|GetSpellObjectMesh))
  (bind _spellobjectmesh_2 (Variables|Default|GetSpellObjectMesh))
  (bind _relativerotation (Variables|/Script/Engine.SceneComponent|GetRelativeRotation _spellobjectmesh))
  (bind (_roll _pitch _yaw) (Math|Rotator|BreakRotator _relativerotation))
  (Class|NiagaraComponent|SetAsset (Variables|Default|GetSpellVFXComponent) (Variables|Default|GetSpellVFX) true)
  (Components|StaticMesh|SetStaticMesh (Variables|Default|GetSpellObjectMesh) (Variables|Default|GetSpellMeshes))
  (Rendering|Material|SetMaterial (Variables|Default|GetSpellObjectMesh) 0 (Variables|Default|GetSpellMaterial))
  (Transformation|SetActorRelativeScale3D (* (Variables|Default|GetRelativeScale) (Variables|Default|GetScale)))
  (Variables|/Script/Engine.ProjectileMovementComponent|SetInitialSpeed (Variables|Default|GetProjectileMovement) (Variables|Default|GetSpeed))
  (Transformation|SetRelativeLocationAndRotation (Variables|Default|GetSpellObjectMesh) (Variables|Default|GetRelativeLocation) (Math|Conversions|RotationFromXVector (+ (Math|Vector|MakeVector _roll _pitch _yaw) (Variables|Default|GetRotation))) false false)
  (Variables|Default|SetStartingLocation (Transformation|GetWorldLocation (Variables|Default|GetDefaultSceneRoot)))
  (if (and (Utilities|Enum|Equal(Enum) (Variables|Default|GetElement) "Earth") (<= (Variables|Default|GetSpeed) 0.0))
    (Collision|SetCollisionProfileName _spellobjectmesh_2 "BlockAll" true :!class /Script/Engine.PrimitiveComponent)
    (Collision|SetCollisionEnabled _spellobjectmesh_2 "QueryAndPhysics")))

(fn SpellObjectTakeDamage
  (params (Damage :type Float%20%28double-precision%29) (DamageDealerHitpoint :type Float%20%28double-precision%29) (Other%20Actor :type BP%20Spell%20Object%20Object%20Reference%20%28by%20ref%29))
  (bind _output_get (Variables|Default|SetHitpoint (- (Variables|Default|GetHitpoint) Damage)))
  (if (> _output_get 0.0)
    (if (> _output_get DamageDealerHitpoint)
      (Development|PrintString (Utilities|String|Append (Variables|Default|GetSurvivedHitDebugString) (Utilities|String|ToString(Float) _output_get)))
      (if (and (> (Variables|Default|GetSpeed) 0.0) (<= (Variables|BP_SpellObject_C|GetSpeed Other%20Actor) 0.0))
        (CallFunction|DestroySelf))
      (else
        (CallFunction|DestroySelf)))
    (else
      (CallFunction|DestroySelf)))
  (return))