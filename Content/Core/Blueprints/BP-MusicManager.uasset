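; Music manager attached to the player character that switches between town, battle and boss music based on nearby enemies.
; MusicSphere overlaps and enemy death events maintain an enemy list and boss flag.
; CheckMusic picks the track and informs the player widget; boss music also requires a non-empty enemy list.
; SetMusic crossfades between pre-created 2D sounds stored in a map, replacing older per-track fade logic left unused.
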(event Custom|OnDeadEvent_Event
  (params (basecharacter :type BP%20Base%20Character%20Object%20Reference))
  (bind _asbp_enemy_aicharacter (Utilities|Casting|CastToBP_EnemyAICharacter basecharacter))
  (Utilities|Array|RemoveItem (Variables|Default|GetEnemyCharacters) _asbp_enemy_aicharacter))

(event Custom|BeginOverlap
  (params (OverlappedComponent :type Primitive%20Component%20Object%20Reference) (OtherActor :type Actor%20Object%20Reference) (OtherComp :type Primitive%20Component%20Object%20Reference) (OtherBodyIndex :type Integer) (bFromSweep :type Boolean) (SweepResult :type Hit%20Result%20Structure%20%28by%20ref%29))
  (CallFunction|CheckMusic)
  (CallFunction|SetMusic)
  (bind _asbp_enemy_aicharacter_boss (Utilities|Casting|CastToBP_EnemyAICharacterBoss OtherActor)
    (:then
      (bind _isdead (Default|IsDead _asbp_enemy_aicharacter_boss))
      (if (not _isdead)
        (Variables|Default|SetIsBoss true)))
    (:CastFailed
      (bind _asbp_enemy_aicharacter (Utilities|Casting|CastToBP_EnemyAICharacter OtherActor))
      (bind _isdead_2 (Default|IsDead _asbp_enemy_aicharacter))
      (if (not (and (not (Utilities|Array|ContainsItem (Variables|Default|GetEnemyCharacters) _asbp_enemy_aicharacter)) _isdead_2))
        (Utilities|Array|Add (Variables|Default|GetEnemyCharacters) _asbp_enemy_aicharacter)
        (EventDispatchers|AssignOnDeadEvent _asbp_enemy_aicharacter (delegate Custom|OnDeadEvent_Event))))))

(event Custom|OnComponentEndOverlap_Event
  (params (OverlappedComponent :type Primitive%20Component%20Object%20Reference) (OtherActor :type Actor%20Object%20Reference) (OtherComp :type Primitive%20Component%20Object%20Reference) (OtherBodyIndex :type Integer))
  (CallFunction|CheckMusic)
  (CallFunction|SetMusic)
  (Utilities|Casting|CastToBP_EnemyAICharacterBoss OtherActor
    (:then
      (Variables|Default|SetIsBoss false))
    (:CastFailed
      (bind _asbp_enemy_aicharacter (Utilities|Casting|CastToBP_EnemyAICharacter OtherActor))
      (Utilities|Array|RemoveItem (Variables|Default|GetEnemyCharacters) _asbp_enemy_aicharacter))))

(event Custom|Check%20and%20play%20music
  ;[1 1 1] PreviousLogic
)

(event EventBeginPlay
  (bind _asbp_camera_controller (Utilities|Casting|CastToBP_CameraController (Game|GetPlayerController 0)))
  (Variables|Default|SetPlayerWidget (Variables|/Game/Characters/Camera/BP_CameraController.BP_CameraController_C|GetPlayerWidget _asbp_camera_controller))
  (bind _returnvalue (Audio|CreateSound2D "/Game/Assets/SFX/Level-SFX/TOWN_SFX.TOWN_SFX" 2.0 1.0 0.0 0 false false))
  (Utilities|Map|Add (Variables|Default|GetMusicMap) "NewEnumerator0" _returnvalue)
  (bind _returnvalue_2 (Audio|CreateSound2D "/Game/Assets/SFX/BOSS_FIGHT_V1.BOSS_FIGHT_V1" 0.8 1.0 0.0 0 false false))
  (Utilities|Map|Add (Variables|Default|GetMusicMap) "NewEnumerator2" _returnvalue_2)
  (bind _returnvalue_3 (Audio|CreateSound2D "/Game/Assets/SFX/BATTLE.BATTLE" 0.8 1.0 0.0 0 false false))
  (Utilities|Map|Add (Variables|Default|GetMusicMap) "NewEnumerator1" _returnvalue_3)
  (bind _asbp_player_character (Utilities|Casting|CastToBP_PlayerCharacter (Components|GetOwner)))
  (Variables|Default|SetOwner _asbp_player_character)
  (Collision|BindEventtoOnComponentBeginOverlap (Variables|/Game/Characters/_Common/Blueprint/BP_PlayerCharacter.BP_PlayerCharacter_C|GetMusicSphere _asbp_player_character) (delegate Custom|BeginOverlap))
  (Collision|AssignOnComponentEndOverlap (Variables|/Game/Characters/_Common/Blueprint/BP_PlayerCharacter.BP_PlayerCharacter_C|GetMusicSphere _asbp_player_character) (delegate Custom|OnComponentEndOverlap_Event))
  (Utilities|Time|SetTimerbyEvent (EventDispatchers|CreateEvent :!event Custom|Check%20and%20play%20music) 1.0 true)
  (for _array_element (Collision|GetOverlappingActors (Variables|/Game/Characters/_Common/Blueprint/BP_PlayerCharacter.BP_PlayerCharacter_C|GetMusicSphere _asbp_player_character) "/Game/Characters/Enemy/Blueprint/BP_EnemyAICharacter.BP_EnemyAICharacter_C" :!class /Script/Engine.PrimitiveComponent)
    (bind _asbp_enemy_aicharacter_boss (Utilities|Casting|CastToBP_EnemyAICharacterBoss _array_element)
      (:then
        (bind _isdead (Default|IsDead _asbp_enemy_aicharacter_boss))
        (if (not _isdead)
          (Variables|Default|SetIsBoss true)
          (EventDispatchers|AssignOnDeadEvent _asbp_enemy_aicharacter_boss (EventDispatchers|CreateEvent :!event Custom|OnDeadEvent_Event))))
      (:CastFailed
        (bind _asbp_enemy_aicharacter (Utilities|Casting|CastToBP_EnemyAICharacter _array_element))
        (bind _isdead_2 (Default|IsDead _asbp_enemy_aicharacter))
        (if (not _isdead_2)
          (Utilities|Array|Add (Variables|Default|GetEnemyCharacters) _asbp_enemy_aicharacter)
          (EventDispatchers|AssignOnDeadEvent _asbp_enemy_aicharacter (EventDispatchers|CreateEvent :!event Custom|OnDeadEvent_Event)))))))

(fn CheckMusic
  (if (Utilities|Array|IsNotEmpty (Variables|Default|GetEnemyCharacters))
    (if (Variables|Default|GetIsBoss)
      (Variables|Default|SetMusic "NewEnumerator2")
      (Default|SetMusic (Variables|Default|GetPlayerWidget) "NewEnumerator2")
      (else
        (Variables|Default|SetMusic "NewEnumerator1")
        (Default|SetMusic (Variables|Default|GetPlayerWidget) "NewEnumerator1")))
    (else
      (Variables|Default|SetMusic "NewEnumerator0")
      (Default|SetMusic (Variables|Default|GetPlayerWidget) "NewEnumerator0"))))

(fn SetMusic
  (bind _musicmap (Variables|Default|GetMusicMap))
  (bind _music (Variables|Default|GetMusic))
  (bind _value (Utilities|Map|Find _musicmap _music))
  (if (not (Audio|Components|Audio|IsPlaying _value))
    (Utilities|IsValid (Variables|Default|GetMusicPlayingCurrently)
      (:Is%20Valid
        (Audio|Components|Audio|FadeOut (Variables|Default|GetMusicPlayingCurrently) 0.5 0.0 "Linear" :!class /Script/Engine.AudioComponent))
      (:Is%20Not%20Valid
        _))
    (bind _output_get (Variables|Default|SetMusicPlayingCurrently _value))
    (Audio|Components|Audio|FadeIn _output_get 0.5 1.0 0.0 "Linear" :!class /Script/Engine.AudioComponent)))