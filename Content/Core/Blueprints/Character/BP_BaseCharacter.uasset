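; Base character shared by player and NPCs, handling stats, damage, healing, death, mana regen and spell attacks.
; The construction script loads stats from a data table keyed by character type and sets up the spell component.
; Alert state and damage source feed the AI blackboard, while damage and death fire dispatchers.
; Tick turns overhead and dialogue widgets toward the camera and triggers ambient dialogue when it is near.
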(event Custom|Hide%20TD%20mesh
  ;[1 1 1] Funcitons we use inside the controller
  (Rendering|SetVisibility (Variables|Character|GetMesh) false false)
  (Rendering|SetVisibility (Variables|Default|GetOverheadWidget) false false))

(event Custom|Show%20TD%20Mesh
  ;[1 1 1] Funcitons we use inside the controller
  (Rendering|SetVisibility (Variables|Character|GetMesh) true false)
  (Rendering|SetVisibility (Variables|Default|GetOverheadWidget) false false))

(event Custom|UpdateAlertState
  (params (Alert%20State :type E_States%20Enum :default "NewEnumerator0"))
  (bind _self self)
  (bind _returnvalue (AI|GetAIController _self))
  ;[1 1 1] Blackboard stuff
  (bind _output_get (Variables|Ai|SetAI%20State Alert%20State))
  (Utilities|IsValid _returnvalue
    (:Is%20Valid
      (AI|Components|Blackboard|SetValueasEnum (AI|GetBlackboard _returnvalue) (Variables|Blackboard|GetStateKey) _output_get))))

(event Custom|Resets%20Character
  (bind _statsdata (Variables|Character|GetStatsData))
  ;[1 1 1] Shared Function By All Characters
  (Variables|Character|SetCurrentHealth (Variables|/Script/GameOff2024.StatsComponent|GetHealthPoint _statsdata))
  (Variables|Character|SetCurrentMana (Variables|/Script/GameOff2024.StatsComponent|GetMana _statsdata))
  (CallFunction|UpdateAlertState "NewEnumerator0")
  (Variables|Widget|GetNPCOverheadWidget ; For NPC
    (:then)
    (:else)))

(event Custom|EnableDecal
  ;[1 1 1] Decal Logic
  (Rendering|SetVisibility (Variables|Default|GetSelectedDecal) true false))

(event Custom|DisableDecal
  ;[1 1 1] Decal Logic
  (Rendering|SetVisibility (Variables|Default|GetSelectedDecal) false false))

(event Custom|OnCameraSwitched
  (params (IsTopDown :type Boolean))
  ;[1 1 1] Decal Logic
  (if (and (not IsTopDown) (Rendering|IsVisible (Variables|Default|GetSelectedDecal)))
    (CallFunction|DisableDecal)))

(event Custom|DisablePawnSensing
  ;[1 1 1] Disable and enable pawn sensing, needed for defend mission trigger
  (Class|PawnSensingComponent|SetSensingUpdatesEnabled (Variables|Default|GetPawnSensing) false))

(event Custom|EnablePawnSensing
  ;[1 1 1] Disable and enable pawn sensing, needed for defend mission trigger
  (Class|PawnSensingComponent|SetSensingUpdatesEnabled (Variables|Default|GetPawnSensing) true))

(event Custom|LockMovement
  ;[1 1 1] Disable and enable pawn sensing, needed for defend mission trigger
  (Variables|Blackboard|SetMovementLockedBeforeMission true)
  (CallFunction|DisablePawnSensing))

(event Custom|UnlockMovement
  ;[1 1 1] Disable and enable pawn sensing, needed for defend mission trigger
  (Variables|Blackboard|SetMovementLockedBeforeMission false)
  (CallFunction|EnablePawnSensing))

(event Custom|Take%20Damage
  (params (Damage :type Float%20%28double-precision%29) (DamageLocation :type Vector))
  ;[1 1 1] Shared Function By All Characters
  (bind _isdead (CallFunction|IsDead))
  (if (not _isdead)
    (bind _output_get (Variables|Character|SetCurrentHealth (Math|Float|Clamp(Float) (- (Variables|Character|GetCurrentHealth) Damage) 0.0 1e+03)))
    (Default|UpdateHealth (Variables|Widget|GetNPCOverheadWidget))
    ;;[0.09273 0.8095 1] Hit Animation
    (Animation|Montage|PlayMontage (Variables|Character|GetMesh) (Variables|Default|GetHitMontageToPlay)
      (:then
        (if (<= _output_get 0.0)
          (CallFunction|OnDeath)
          (else
            (CallFunction|SetLastDamageLocation DamageLocation))))
      (:OnNotifyBegin
        (Audio|PlaySoundatLocation (Variables|Default|GetSoundToPlayOnHit) (Transformation|GetActorLocation) "0, 0, 0" 0.4 1.0 0.0 0 0 0 0)))))

(event Custom|OnDeath
  (bind _deathanimation (Variables|Animation|GetDeathAnimation))
  ;[1 1 1] Shared Function By All Characters
  (CallFunction|DisablePawnSensing)
  (CallFunction|UpdateAlertState "NewEnumerator3")
  (Default|CallOnDeadEvent self)
  ;;[0 0.9227 1] DeathAnimation
  (Utilities|IsValid _deathanimation
    (:Is%20Valid
      (Animation|Montage|PlayMontage (Variables|Character|GetMesh) _deathanimation
        (:OnCompleted
          (Actor|DestroyActor :!label _label))
        (:OnBlendOut
          (goto _label))
        (:OnNotifyBegin
          (Audio|PlaySoundatLocation (Variables|Default|GetDeathSound) (Transformation|GetActorLocation) "0, 0, 0" 1.0 1.0 0.0 0 0 0 0)
          (Default|StopAmbiantDialogue (Variables|Widget|GetNPCDialogueWidget))
          (Utilities|FlowControl|Delay 3.0)
          (Actor|DestroyActor :!label _label_2))))
    (:Is%20Not%20Valid
      (goto _label_2))))

(event Custom|Attack
  ;[1 1 1] Shared Function By All Characters
  ;;[1 1 1] Shoot Magic
  (if (not (Variables|Character|GetIsPlayer))
    ;;;[0 1 0.9915] Spell Animation
    (Animation|Montage|PlayMontage (Variables|Character|GetMesh) (Variables|Animation|GetSpellCastMontage) :!label _label
      (:OnNotifyBegin
        (Default|ShootProjectile (Variables|Default|GetSpellComponent) (Transformation|GetWorldTransform (Variables|Default|GetMagic%20Muzzle)))))
    (elif (Variables|Default|GetISTopdown?)
      (goto _label)
      (else
        (Default|ShootProjectile (Variables|Default|GetSpellComponent) (Transformation|GetWorldTransform (Variables|Default|GetMagic%20Muzzle)))))))

(event Custom|Print%20Stats
  (bind _statsdata (Variables|Character|GetStatsData))
  ;[1 1 1] Debug Print For Stats
  (Development|PrintString (Utilities|String|Append "Health Point: " (Utilities|String|ToString(Float) (Variables|/Script/GameOff2024.StatsComponent|GetHealthPoint _statsdata)) " 
Mana: " (Utilities|String|ToString(Float) (Variables|/Script/GameOff2024.StatsComponent|GetMana _statsdata)) " 
Mana Regen:" (Utilities|String|ToString(Float) (Variables|/Script/GameOff2024.StatsComponent|GetManaRegenerationRate _statsdata)) " 
Character Type" (Utilities|String|EnumtoString (Variables|Character|GetCharacter%20Type)))))

(event Custom|Load%20From%20Data%20Table
  (bind _statsdata (Variables|Character|GetStatsData))
  ;[1 1 1] Read Stats From Data Table (done in construction script)
  (bind _returnvalue (Utilities|GetDataTableRow "/Game/Core/Blueprints/Character/UnitInfoDataTable.UnitInfoDataTable" (Utilities|String|StringToName (Utilities|String|EnumtoString (Variables|Character|GetCharacter%20Type))))
    (:then
      (Variables|Character|SetName (.Name (Utilities|Struct|BreakUnitInfo _returnvalue)))
      (Variables|Default|SetDescription (.Description (Utilities|Struct|BreakUnitInfo _returnvalue)))
      (Variables|Character|SetCharacter%20Type (.CharacterType (Utilities|Struct|BreakUnitInfo _returnvalue)))
      (bind _output_get (Variables|/Script/GameOff2024.StatsComponent|SetHealthPoint _statsdata (.HealthPoint (Utilities|Struct|BreakUnitInfo _returnvalue))))
      (Variables|Character|SetCurrentHealth _output_get)
      (Variables|/Script/GameOff2024.StatsComponent|SetSkill _statsdata (.Skill (Utilities|Struct|BreakUnitInfo _returnvalue)))
      (Variables|/Script/GameOff2024.StatsComponent|SetMovementSpeed _statsdata (.MovementSpeed (Utilities|Struct|BreakUnitInfo _returnvalue)))
      (bind _output_get_2 (Variables|/Script/GameOff2024.StatsComponent|SetMana _statsdata (.Mana (Utilities|Struct|BreakUnitInfo _returnvalue))))
      (Variables|Character|SetCurrentMana _output_get_2)
      (Variables|/Script/GameOff2024.StatsComponent|SetManaRegenerationRate _statsdata (.ManaRegen (Utilities|Struct|BreakUnitInfo _returnvalue))))
    (:RowNotFound
      (Development|PrintString (Utilities|String|Append (Utilities|String|EnumtoString (Variables|Character|GetCharacter%20Type)) " Unit Type Not Found, Please Create One")))))

(event Custom|Set%20Last%20Damage%20Location
  (params (Damage%20Location :type Vector))
  ;[1 1 1] Blackboard stuff
  (Default|CallOnDamageEvent Damage%20Location)
  (CallFunction|InformBlackboardDamageSourceLocation Damage%20Location))

(event Custom|Heal
  (params (Heal%20Amount :type Float%20%28double-precision%29))
  ;[1 1 1] Shared Function By All Characters
  (bind _isdead (CallFunction|IsDead))
  (if (not _isdead)
    (Variables|Character|SetCurrentHealth (Math|Float|Clamp(Float) (+ (Variables|Character|GetCurrentHealth) Heal%20Amount) 0.0 (Variables|/Script/GameOff2024.StatsComponent|GetHealthPoint (Variables|Character|GetStatsData))))
    (bind _npcoverheadwidget (Variables|Widget|GetNPCOverheadWidget) ; For NPC
      (:then
        (Default|UpdateHealth _npcoverheadwidget)
        (if (Variables|Character|GetIsPlayer)
          (bind _asbp_camera_controller (Utilities|Casting|CastToBP_CameraController (Game|GetPlayerController 0)))
          (Default|UpdateHealthUI (Variables|/Game/Core/Blueprints/Character/BP_CameraController.BP_CameraController_C|GetPlayerWidget _asbp_camera_controller))))
      (:else))))

(event Custom|InformBlackboardDamageSourceLocation
  (params (LastDamageLocation :type Vector))
  (bind _self self)
  (bind _returnvalue (AI|GetAIController _self))
  ;[1 1 1] Blackboard stuff
  (Variables|Default|SetDamageSourceToReactTo true)
  (Variables|Ai|SetLastDamageLocation LastDamageLocation)
  (Utilities|IsValid _returnvalue
    (:Is%20Valid
      (AI|Components|Blackboard|SetValueasVector (AI|GetBlackboard _returnvalue) (Variables|Blackboard|GetDamageSourceLocationKey) (Variables|Ai|GetLastDamageLocation))
      (CallFunction|UpdateAlertState "NewEnumerator1"))))

(event EventTick
  (params (DeltaSeconds :type Float%20%28single-precision%29))
  (bind _returnvalue (Game|GetPlayerCameraManager 0))
  (bind _dialoguewidget (Variables|Default|GetDialogueWidget))
  (bind _npcdialoguewidget (Variables|Widget|GetNPCDialogueWidget))
  (bind _overheadwidget (Variables|Default|GetOverheadWidget))
  (bind _returnvalue_2 (Transformation|GetWorldLocation _overheadwidget))
  (bind _returnvalue_3 (Transformation|GetWorldLocation _dialoguewidget))
  (bind _transformcomponent (Variables|/Script/Engine.PlayerCameraManager|GetTransformComponent _returnvalue))
  (bind _returnvalue_4 (Transformation|GetWorldLocation _transformcomponent))
  (bind _returnvalue_5 (Math|Rotator|FindLookatRotation _returnvalue_2 _returnvalue_4))
  (bind _returnvalue_6 (Math|Rotator|FindLookatRotation _returnvalue_3 _returnvalue_4))
  ;[1 1 1] Event Tick
  ;;[1 1 1] Rotate Widget
  (Transformation|SetWorldRotation _overheadwidget (Math|Rotator|MakeRotator (.roll _returnvalue_5) 0.0 (.yaw _returnvalue_5)) false false) ; rotate widget to face player
  (Transformation|SetWorldRotation _dialoguewidget (Math|Rotator|MakeRotator (.roll _returnvalue_6) 0.0 (.yaw _returnvalue_6)) false false) ; rotate widget to face player
  (bind _isdead (CallFunction|IsDead))
  (if (not _isdead) ; Only update if it is not dead
    (if (and (<= (Math|Vector|Distance(Vector) (Transformation|GetActorLocation (Game|GetPlayerCameraManager 0)) (Transformation|GetWorldLocation (Variables|Collision|GetCapsuleComponent self))) (Variables|Default|GetRangeConsideredNearPlayer)) (not (Variables|Character|GetIsInteracting)))
      (Default|StartAmbiantDialogue _npcdialoguewidget (Variables|Ai|GetAI%20State))
      (else
        (Default|StopAmbiantDialogue _npcdialoguewidget)))
    ;;[1 1 1] Mana Regen
    (if (< (Variables|Character|GetCurrentMana) (Variables|/Script/GameOff2024.StatsComponent|GetMana (Variables|Character|GetStatsData)))
      (Variables|Character|SetCurrentMana (Math|Float|Clamp(Float) (+ (Variables|Character|GetCurrentMana) (* (Variables|/Script/GameOff2024.StatsComponent|GetManaRegenerationRate (Variables|Character|GetStatsData)) DeltaSeconds)) 0.0 1e+02))
      (bind _npcoverheadwidget (Variables|Widget|GetNPCOverheadWidget)
        (:then
          (Default|UpdateMana _npcoverheadwidget))
        (:else)))))

(event EventBeginPlay
  (bind _self self)
  (bind _returnvalue (AI|GetAIController _self))
  ;[1 1 1] Begin Play Load the Widget
  (bind _asbp_enemy_overhead_widget (Utilities|Casting|CastToBP_EnemyOverheadWidget (UserInterface|GetWidget (Variables|Default|GetOverheadWidget))))
  (bind _output_get (Variables|Widget|SetNPCOverheadWidget _asbp_enemy_overhead_widget))
  (Default|LoadfromCharacter _output_get self)
  (bind _returnvalue_2 (Game|ConstructObjectfromClass "/Game/UI/BP_DialogueOverHeadWidget.BP_DialogueOverHeadWidget_C" self))
  (bind _output_get_2 (Variables|Widget|SetNPCDialogueWidget _returnvalue_2))
  (UserInterface|SetWidget (Variables|Default|GetDialogueWidget) _output_get_2)
  (Rendering|SetCastShadow (Variables|Default|GetOverheadWidget) false)
  (Rendering|SetCastShadow (Variables|Default|GetDialogueWidget) false)
  (bind _asbp_camera_controller (Utilities|Casting|CastToBP_CameraController (Game|GetPlayerController 0)))
  (EventDispatchers|BindEventtoOnCameraSwitched _asbp_camera_controller (EventDispatchers|CreateEvent :!event Custom|OnCameraSwitched))
  (bind _output_get_3 (Variables|Ai|SetInitialLocation (Transformation|GetActorLocation))) ; Set Initial Location so enemy will go back to original location
  (Utilities|IsValid _returnvalue
    (:Is%20Valid
      (AI|Components|Blackboard|SetValueasVector (AI|GetBlackboard _returnvalue) (Variables|Blackboard|GetInitialLocationKey) _output_get_3))))

(fn ConstructionScript
  (bind _statsdata (Variables|Character|GetStatsData))
  (Default|LoadfromDataTable (Variables|Default|GetSpellComponent))
  (CallFunction|LoadfromDataTable)
  (Variables|Character|SetCurrentHealth (Variables|/Script/GameOff2024.StatsComponent|GetHealthPoint _statsdata))
  (Variables|Character|SetCurrentMana (Variables|/Script/GameOff2024.StatsComponent|GetMana _statsdata))
  (CallFunction|SetMovementSpeed "NewEnumerator2"))

(fn StartSprinting
  (Variables|/Script/Engine.CharacterMovementComponent|SetMaxWalkSpeed (Variables|Character|GetCharacterMovement) (Variables|Playermovement|GetSprintSpeed)))

(fn StopSprinting
  (Variables|/Script/Engine.CharacterMovementComponent|SetMaxWalkSpeed (Variables|Character|GetCharacterMovement) (Variables|PlayerMovement|GetWalkSpeed)))

(fn IsDead
  (return (Utilities|Enum|Equal(Enum) (Variables|Ai|GetAI%20State) "NewEnumerator3")))

(fn IsAttacking
  (bind _ai_state (Variables|Ai|GetAI%20State))
  (return (or (Utilities|Enum|Equal(Enum) _ai_state "NewEnumerator1") (Utilities|Enum|Equal(Enum) _ai_state "NewEnumerator2"))))

(fn GetPatrolRoute
  (return (Variables|Ai|GetPatrol)))

(fn SetMovementSpeed
  (params (Speed :type E_Speed%20Enum :default "NewEnumerator0"))
  (bind _output_get (Variables|/Script/Engine.CharacterMovementComponent|SetMaxWalkSpeed (Variables|Character|GetCharacterMovement) (Utilities|Select :Index Speed :NewEnumerator0 0.0 :NewEnumerator1 1e+02 :NewEnumerator2 (Variables|/Script/GameOff2024.StatsComponent|GetMovementSpeed (Variables|Character|GetStatsData)))))
  (return _output_get))