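; Player character Blueprint that shows a game over screen and plays a sound on death, and can act as an AI-controlled ally.
; Under an ally AI controller, pawn sensing feeds enemy targets to that controller, raises a one-time detection event and drops targets through a retriggerable delay.
; A sphere overlap tracks InteractInterface actors and toggles the HUD prompt, and PlayerInteract messages the stored actor.
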(event OnComponentBeginOverlap(Sphere)
  (params (OverlappedComponent :type Primitive%20Component%20Object%20Reference) (OtherActor :type Actor%20Object%20Reference) (OtherComp :type Primitive%20Component%20Object%20Reference) (OtherBodyIndex :type Integer) (bFromSweep :type Boolean) (SweepResult :type Hit%20Result%20Structure%20%28by%20ref%29))
  ;[1 1 1] Interact
  (if (Utilities|DoesObjectImplementInterface OtherActor "/Game/Core/Blueprints/Item/InteractInterface.InteractInterface_C")
    (Variables|Default|SetOverlapActor OtherActor)
    (bind _asbp_camera_controller (Utilities|Casting|CastToBP_CameraController (Game|GetPlayerController 0)))
    (Default|DisplayInteractText (Variables|/Game/Core/Blueprints/Character/BP_CameraController.BP_CameraController_C|GetPlayerWidget _asbp_camera_controller))))

(event OnSeePawn(PawnSensing)
  (params (Pawn :type Pawn%20Object%20Reference))
  (bind _self self)
  (bind _returnvalue (AI|GetAIController _self))
  ;[1 1 1] Pawn Sensing when Controller is AI
  (Utilities|IsValid _returnvalue
    (:Is%20Valid
      (bind _asbp_ally_aicontroller (Utilities|Casting|CastToBP_AllyAIController _returnvalue))
      (bind _asbp_enemy_aicharacter (Utilities|Casting|CastToBP_EnemyAICharacter Pawn))
      (if (Utilities|Enum|NotEqual(Enum) (Variables|/Game/Core/Blueprints/Character/BP_BaseCharacter.BP_BaseCharacter_C|GetAI%20State _asbp_enemy_aicharacter) "NewEnumerator3")
        (bind _output_get (Variables|Default|SetCurrentTarget _asbp_enemy_aicharacter))
        (Utilities|FlowControl|Sequence ; This to reset the delay if we keep seeing the enemy
          (:then_0
            (Development|PrintString "Enemy Update")
            (Default|OnPerceptionActorUpdated _asbp_ally_aicontroller _output_get)
            (if (not (Variables|Default|GetHasInformNPC))
              (Default|CallOnEnemyDetectedEvent (Transformation|GetWorldLocation (Variables|/Script/Engine.Character|GetCapsuleComponent _output_get)))
              (Variables|Default|SetHasInformNPC true)))
          (:then_1
            (Utilities|FlowControl|RetriggerableDelay 2.0) ; Only Lose Target After x second
            (Default|OnPerceptionActorUpdated _asbp_ally_aicontroller)))))))

(event OnComponentEndOverlap(Sphere)
  (params (OverlappedComponent :type Primitive%20Component%20Object%20Reference) (OtherActor :type Actor%20Object%20Reference) (OtherComp :type Primitive%20Component%20Object%20Reference) (OtherBodyIndex :type Integer))
  ;[1 1 1] Interact
  (if (Utilities|DoesObjectImplementInterface OtherActor "/Game/Core/Blueprints/Item/InteractInterface.InteractInterface_C")
    (Variables|Default|SetOverlapActor OtherActor)
    (bind _asbp_camera_controller (Utilities|Casting|CastToBP_CameraController (Game|GetPlayerController 0)))
    (Default|HideInteractText (Variables|/Game/Core/Blueprints/Character/BP_CameraController.BP_CameraController_C|GetPlayerWidget _asbp_camera_controller))))

(event Custom|PlayerInteract
  (bind _overlapactor (Variables|Default|GetOverlapActor))
  ;[1 1 1] Interact
  (Utilities|IsValid _overlapactor
    (:Is%20Valid
      (Class|InteractInterface|Interact(Message) _overlapactor self))))

(event EventBeginPlay
  (|CallParentFunction)
  (UserInterface|SetWidget (Variables|Default|GetDialogueWidget) 0) ; Remove the dialogue overhead widget since player doesn't need it
)

(event EventOnCameraSwitched
  (params (IsTopDown :type Boolean))
  (|CallParentFunction IsTopDown)
  (CallFunction|SetMovementSpeed "NewEnumerator2"))

(event EventOnDeath
  ;[1 1 1] Game Over Condition for player
  ;[1 1 1] Test (create game over screen)
  (|CallParentFunction)
  (bind _returnvalue (UserInterface|CreateWidget "/Game/UI/BP_GameOverScreen.BP_GameOverScreen_C"))
  (UserInterface|Viewport|AddtoViewport _returnvalue 0)
  (Audio|PlaySoundatLocation "/Game/Assets/SFX/Player-SFX/Sounds/Sound/PlayerDeathSFX/DEATH_SFX.DEATH_SFX" (Transformation|GetWorldLocation (Variables|Default|GetCapsuleComponent)) "0, 0, 0" 1.0 1.0 0.0 0 0 0 0))

(fn ConstructionScript
  (|CallParentFunction))

(fn SetMovementSpeed
  (params (Speed :type E_Speed%20Enum :default "NewEnumerator0"))
  (return 0.0))