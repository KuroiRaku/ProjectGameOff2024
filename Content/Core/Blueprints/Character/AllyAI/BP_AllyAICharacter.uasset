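; Ally NPC character that spots enemies, talks to the player and can join them as a follower.
; Pawn sensing passes living allies' targets to BP_AllyAIController and raises a one-shot detection event, with a retriggerable delay clearing target and alert after sight is lost.
; Interacting halts and focuses the ally for dialogue; past a dialogue index, eligible allies join through the controller, which can also happen at BeginPlay.
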(event OnSeePawn(PawnSensing)
  (params (Pawn :type Pawn%20Object%20Reference))
  (bind _isdead (CallFunction|IsDead))
  (if (not _isdead)
    (bind _asbp_enemy_aicharacter (Utilities|Casting|CastToBP_EnemyAICharacter Pawn))
    (if (Utilities|Enum|NotEqual(Enum) (Variables|/Game/Core/Blueprints/Character/BP_BaseCharacter.BP_BaseCharacter_C|GetAI%20State _asbp_enemy_aicharacter) "NewEnumerator3")
      (bind _output_get (Variables|Default|SetCurrentTarget _asbp_enemy_aicharacter))
      (Utilities|FlowControl|Sequence ; This to reset the delay if we keep seeing the enemy
        (:then_0
          (Default|OnPerceptionActorUpdated (Variables|Default|GetAllyAIController) _output_get)
          (if (not (Variables|Default|GetHasInformNPC))
            (Default|CallOnEnemyDetectedEvent (Transformation|GetWorldLocation (Variables|/Script/Engine.Character|GetCapsuleComponent _output_get)))
            (Variables|Default|SetHasInformNPC true)))
        (:then_1
          (Utilities|FlowControl|RetriggerableDelay 5.0) ; Only Lose Target After x second
          (bind _isdead_2 (CallFunction|IsDead))
          (if (not _isdead_2)
            (Default|OnPerceptionActorUpdated (Variables|Default|GetAllyAIController))
            (Variables|Default|SetHasInformNPC false)
            (CallFunction|UpdateAlertState "NewEnumerator0")))))))

(event Custom|FollowPlayer
  (bind _allyaicontroller (Variables|Default|GetAllyAIController))
  (bind _asbp_camera_controller (Utilities|Casting|CastToBP_CameraController (Game|GetPlayerController 0)))
  (bind _player_character (Variables|/Game/Core/Blueprints/Character/BP_CameraController.BP_CameraController_C|GetPlayer%20Character _asbp_camera_controller)
    (:then
      (Default|JoinPlayer _allyaicontroller _player_character))
    (:else
      (bind _asbp_player_character (Utilities|Casting|CastToBP_PlayerCharacter (Game|GetPlayerCharacter 0)))
      (Default|JoinPlayer _allyaicontroller _asbp_player_character)))
  (Variables|Default|SetIsHostage false)
  (Variables|Default|SetJoinedPlayer true))

(event EventBeginPlay
  (|CallParentFunction)
  (bind _asbp_ally_aicontroller (Utilities|Casting|CastToBP_AllyAIController (Pawn|GetController)))
  (Variables|Default|SetAllyAIController _asbp_ally_aicontroller)
  (if (Variables|Default|GetJoinPlayerAtStart)
    (CallFunction|FollowPlayer)))

(event EventInteract
  (params (Character :type BP%20Base%20Character%20Object%20Reference))
  (bind _self self)
  (bind _returnvalue (AI|GetAIController _self))
  ;[1 1 1] Interacting
  (CallFunction|LockMovement)
  (AI|Navigation|StopMovement _returnvalue)
  (AI|SetFocus _returnvalue Character)
  (bind _npcdialoguewidget (Variables|Default|GetNPCDialogueWidget)
    (:then
      (Default|InteractMessage _npcdialoguewidget (Variables|Default|GetAI%20State))
      (Variables|Default|SetIsInteracting true)
      (if (Math|Boolean|ANDBoolean (> (Variables|/Game/UI/BP_DialogueOverHeadWidget.BP_DialogueOverHeadWidget_C|GetIdleInteractDialogueIndex _npcdialoguewidget) 1) (not (Variables|Default|GetJoinedPlayer)) (Variables|Default|GetAbleToJoinPlayer))
        (CallFunction|FollowPlayer)
        (Utilities|FlowControl|RetriggerableDelay 1.0) ; Stop for at least 5 seconds
        (AI|ClearFocus _returnvalue)
        (CallFunction|UnlockMovement)
        (Variables|Default|SetIsInteracting false)))
    (:else)))

(fn ConstructionScript
  (|CallParentFunction))

(fn GetObjectName
  (return ""))