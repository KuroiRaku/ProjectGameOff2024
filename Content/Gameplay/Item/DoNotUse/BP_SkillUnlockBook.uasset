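; Interactable skill book that unlocks spell-crafting options for the character that uses it.
; On Interact, it checks its configured spell slot, element, shape, speed and size against the progression maps on the character's SpellComponent, setting any locked entry to true.
; Newly unlocked enum names accumulate in LearnedMessage, which is printed as debug text for a player with BP_CameraController, or an already-learned notice if empty.
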(event EventInteract
  (params (Character :type BP%20Base%20Character%20Object%20Reference))
  (bind _spellcomponent (Variables|/Game/Characters/_Common/Blueprint/BP_BaseCharacter.BP_BaseCharacter_C|GetSpellComponent Character))
  (bind _unlock (Variables|Default|GetUnlock))
  (bind _unlockspellslot (Variables|Default|GetUnlockSpellSlot))
  (bind _spellslotprogression (Variables|/Game/Gameplay/Magic/MagicComponent/BP_SpellComponent.BP_SpellComponent_C|GetSpellSlotProgression _spellcomponent))
  (bind _elementtypeprogressionmap (Variables|/Game/Gameplay/Magic/MagicComponent/BP_SpellComponent.BP_SpellComponent_C|GetElementTypeProgressionMap _spellcomponent))
  (bind _sizetypeprogression (Variables|/Game/Gameplay/Magic/MagicComponent/BP_SpellComponent.BP_SpellComponent_C|GetSizeTypeProgression _spellcomponent))
  (bind _speedtypeprogressionmap (Variables|/Game/Gameplay/Magic/MagicComponent/BP_SpellComponent.BP_SpellComponent_C|GetSpeedTypeProgressionMap _spellcomponent))
  (bind _shapetypeprogression (Variables|/Game/Gameplay/Magic/MagicComponent/BP_SpellComponent.BP_SpellComponent_C|GetShapeTypeProgression _spellcomponent))
  (Utilities|IsValid Character
    (:Is%20Valid
      ;[1 1 1] Check Spell Slot to Unlock
      (if (.Value (Utilities|Map|Find _spellslotprogression _unlockspellslot))
        _
        (else
          (Utilities|Map|Add _spellslotprogression _unlockspellslot true)
          (Variables|Default|SetLearnedMessage (Utilities|String|Append (Utilities|String|EnumtoString _unlockspellslot) ", " (Variables|Default|GetLearnedMessage)))))
      (if (.Value (Utilities|Map|Find _elementtypeprogressionmap (.element _unlock)))
        _
        (else
          (Utilities|Map|Add _elementtypeprogressionmap (.element _unlock) true)
          (Variables|Default|SetLearnedMessage (Utilities|String|Append (Utilities|String|EnumtoString (.element _unlock)) ", " (Variables|Default|GetLearnedMessage)))))
      (if (.Value (Utilities|Map|Find _shapetypeprogression (.shape _unlock)))
        _
        (else
          (Utilities|Map|Add _shapetypeprogression (.shape _unlock) true)
          (Variables|Default|SetLearnedMessage (Utilities|String|Append (Utilities|String|EnumtoString (.shape _unlock)) ", " (Variables|Default|GetLearnedMessage)))))
      (if (.Value (Utilities|Map|Find _speedtypeprogressionmap (.speed _unlock)))
        _
        (else
          (Utilities|Map|Add _speedtypeprogressionmap (.speed _unlock) true)
          (Variables|Default|SetLearnedMessage (Utilities|String|Append (Utilities|String|EnumtoString (.speed _unlock)) ", " (Variables|Default|GetLearnedMessage)))))
      (if (.Value (Utilities|Map|Find _sizetypeprogression (.size _unlock)))
        _
        (else
          (Utilities|Map|Add _sizetypeprogression (.size _unlock) true)
          (Variables|Default|SetLearnedMessage (Utilities|String|Append (Utilities|String|EnumtoString (.size _unlock)) ", " (Variables|Default|GetLearnedMessage)))))
      (bind _asbp_player_character (Utilities|Casting|CastToBP_PlayerCharacter Character))
      (bind _asbp_camera_controller (Utilities|Casting|CastToBP_CameraController (Pawn|GetController _asbp_player_character))
        (:then
          (if (Utilities|Array|IsEmpty (Variables|Default|GetLearnedMessage))
            (Development|PrintString "You have already learned from this book")
            (else
              (Development|PrintString (Utilities|String|Append "You have learned " (.LeftS (Utilities|String|Split (Variables|Default|GetLearnedMessage) "," "IgnoreCase" "FromEnd")))))))
        (:CastFailed
          (Development|PrintString "Invalid Controller?"))))))

(fn ConstructionScript)

(fn GetObjectName
  (return ""))