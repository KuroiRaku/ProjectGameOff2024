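; BP_Mission is a level mission actor that tracks one objective type (Kill Boss, Route, Hostage, Escape or Defend) and reports success or failure once.
; BeginPlay binds character death, damage and detection events, which drive per-type evaluation and threat alerts among mission enemies.
; Its MissionVolume completes Escape on player entry and updates hostages on exit.
; Defend freezes participants until StartMission unlocks them and targets enemies on the protected character.
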(event OnComponentEndOverlap(MissionVolume)
  (params (OverlappedComponent :type Primitive%20Component%20Object%20Reference) (OtherActor :type Actor%20Object%20Reference) (OtherComp :type Primitive%20Component%20Object%20Reference) (OtherBodyIndex :type Integer))
  (bind _asbp_base_character (Utilities|Casting|CastToBP_BaseCharacter OtherActor))
  (if (Utilities|Array|ContainsItem (Variables|Default|GetHostages) _asbp_base_character)
    (Utilities|Array|RemoveItem (Variables|Default|GetHostages) _asbp_base_character)
    (CallFunction|UpdateMission)))

(event OnComponentBeginOverlap(MissionVolume)
  (params (OverlappedComponent :type Primitive%20Component%20Object%20Reference) (OtherActor :type Actor%20Object%20Reference) (OtherComp :type Primitive%20Component%20Object%20Reference) (OtherBodyIndex :type Integer) (bFromSweep :type Boolean) (SweepResult :type Hit%20Result%20Structure%20%28by%20ref%29))
  (Utilities|Casting|CastToBP_PlayerCharacter OtherActor)
  (switch Utilities|FlowControl|Switch|SwitchonE_MissionType (Variables|Default|GetMissionType)
    (:NewEnumerator3
      (CallFunction|CompleteMission true))))

(event Custom|InformAllyOnThreat
  (params (Location :type Vector))
  (for _array_element (Variables|Default|GetEnemyToDefeat)
    (Default|InformBlackboardDamageSourceLocation _array_element Location)))

(event Custom|StartMission
  ;[1 1 1] Only For Defend Mission
  (if (Utilities|Enum|Equal(Enum) (Variables|Default|GetMissionType) "NewEnumerator4")
    (bind _charactertoprotect (Variables|Default|GetCharacterToProtect)
      (:then
        (for _array_element (Variables|Default|GetEnemyToDefeat)
          (Default|SetTarget _array_element _charactertoprotect)
          (Default|UnlockMovement _array_element))
        (Default|UnlockMovement (Variables|Default|GetCharacterToProtect)))
      (:else))))

(event Custom|UpdateMission
  (params (Character :type BP%20Base%20Character%20Object%20Reference))
  (switch Utilities|FlowControl|Switch|SwitchonE_MissionType (Variables|Default|GetMissionType)
    (:NewEnumerator0
      (CallFunction|EvaluateBossMission))
    (:NewEnumerator1
      (CallFunction|EvaluateRouteMission))
    (:NewEnumerator2
      (CallFunction|EvaluateHostageMission))
    (:NewEnumerator4
      (CallFunction|EvaluateDefendMission))))

(event Custom|CompleteMission
  (params (IsSuccessful :type Boolean))
  (if (not (Variables|Default|GetCompleted))
    (Variables|Default|SetCompleted true)
    (Default|CallMissionComplete self IsSuccessful)))

(event EventBeginPlay
  (bind _charactertoprotect (Variables|Default|GetCharacterToProtect))
  (bind _asbp_camera_controller (Utilities|Casting|CastToBP_CameraController (Game|GetPlayerController 0)))
  (Variables|Default|SetPlayerController _asbp_camera_controller)
  (switch Utilities|FlowControl|Switch|SwitchonE_MissionType (Variables|Default|GetMissionType)
    (:NewEnumerator0
      (EventDispatchers|BindEventtoOnDeadEvent (Variables|Default|GetBossToDefeat) (EventDispatchers|CreateEvent :!event Custom|UpdateMission)))
    (:NewEnumerator1
      _)
    (:NewEnumerator2
      (for _array_element (Variables|Default|GetHostages)
        (EventDispatchers|BindEventtoOnDeadEvent _array_element (EventDispatchers|CreateEvent :!event Custom|UpdateMission))
        (bind _asbp_ally_aicharacter (Utilities|Casting|CastToBP_AllyAICharacter _array_element))
        (Variables|/Game/Characters/Ally/Blueprint/BP_AllyAICharacter.BP_AllyAICharacter_C|SetIsHostage _asbp_ally_aicharacter true)))
    (:NewEnumerator3
      _)
    (:NewEnumerator4
      (EventDispatchers|BindEventtoOnDeadEvent _charactertoprotect (EventDispatchers|CreateEvent :!event Custom|UpdateMission))
      (Default|LockMovement _charactertoprotect)
      (for _array_element_2 (Variables|Default|GetEnemyToDefeat) ; Not optimized
        (Default|LockMovement _array_element_2))))
  (for _array_element_3 (Variables|Default|GetEnemyToDefeat)
    (EventDispatchers|BindEventtoOnDeadEvent _array_element_3 (EventDispatchers|CreateEvent :!event Custom|UpdateMission))
    (EventDispatchers|BindEventtoOnDamageEvent _array_element_3 (EventDispatchers|CreateEvent :!event Custom|InformAllyOnThreat))
    (EventDispatchers|BindEventtoOnEnemyDetectedEvent _array_element_3 (EventDispatchers|CreateEvent :!event Custom|InformAllyOnThreat))
    (Variables|/Game/Characters/_Common/Blueprint/BP_BaseCharacter.BP_BaseCharacter_C|SetMissionAssigned _array_element_3 self)))

(fn ConstructionScript)

(fn EvaluateRouteMission
  (bind _enemytodefeat (Variables|Default|GetEnemyToDefeat))
  (if (Utilities|Array|IsNotEmpty _enemytodefeat)
    (bind _arrayelement (Utilities|Array|ReverseforEachLoop _enemytodefeat)
      (:LoopBody
        (bind _isdead (Default|IsDead _arrayelement))
        (if _isdead
          (Utilities|Array|RemoveItem _enemytodefeat _arrayelement)))
      (:Completed
        (if (Utilities|Array|IsEmpty (Variables|Default|GetEnemyToDefeat))
          (CallFunction|CompleteMission true))))
    (else
      (CallFunction|CompleteMission true))))

(fn EvaluateHostageMission
  (bind _enemytodefeat (Variables|Default|GetEnemyToDefeat))
  (if (Utilities|Array|IsNotEmpty _enemytodefeat)
    (bind _arrayelement (Utilities|Array|ReverseforEachLoop _enemytodefeat)
      (:LoopBody
        (bind _isdead (Default|IsDead _arrayelement))
        (if _isdead
          (Utilities|Array|RemoveItem _enemytodefeat _arrayelement)))
      (:Completed
        (bind _arrayelement_2 (Utilities|Array|ReverseforEachLoop (Variables|Default|GetHostages))
          (:LoopBody
            (bind _isdead_2 (Default|IsDead _arrayelement_2))
            (if _isdead_2
              (CallFunction|CompleteMission false) ; Fail Mission If Hostage Is Dead
              (else
                (Utilities|Array|RemoveItem (Variables|Default|GetHostages) _arrayelement_2))))
          (:Completed
            (if (or (<= (Utilities|Array|Length (Variables|Default|GetHostages)) 0) (<= (Utilities|Array|Length (Variables|Default|GetEnemyToDefeat)) 0))
              (CallFunction|CompleteMission true))))))
    (else
      (CallFunction|CompleteMission true))))

(fn EvaluateBossMission
  (bind _bosstodefeat (Variables|Default|GetBossToDefeat))
  (Utilities|IsValid _bosstodefeat
    (:Is%20Valid
      (bind _isdead (Default|IsDead _bosstodefeat))
      (if _isdead
        (CallFunction|CompleteMission true :!label _label)))
    (:Is%20Not%20Valid
      (Development|PrintString "Not Valid, mission succeed Automatically")
      (goto _label))))

(fn WithinBound
  (params (Actor :type Actor%20Object%20Reference) (Container :type Actor%20Object%20Reference))
  (bind (_origin _boxextent) (Collision|GetActorBounds Container false false))
  (bind _returnvalue (Transformation|GetActorLocation Actor))
  (bind (_x _y _z) (Math|Vector|BreakVector _origin))
  (bind (_x_2 _y_2 _z_2) (Math|Vector|BreakVector _boxextent))
  (if (Math|Boolean|ANDBoolean (>= _x (.x _returnvalue)) (>= _y (.y _returnvalue)) (>= _z (.z _returnvalue)) (<= (.x _returnvalue) _x_2) (<= (.y _returnvalue) _y_2) (<= (.z _returnvalue) _z_2))
    (return true)
    (else
      (return false))))

(fn EvaluateDefendMission
  (bind _enemytodefeat (Variables|Default|GetEnemyToDefeat))
  (if (Utilities|Array|IsNotEmpty _enemytodefeat)
    (bind _arrayelement (Utilities|Array|ReverseforEachLoop _enemytodefeat)
      (:LoopBody
        (bind _isdead (Default|IsDead _arrayelement))
        (if _isdead
          (Utilities|Array|RemoveItem _enemytodefeat _arrayelement)))
      (:Completed
        (bind _charactertoprotect (Variables|Default|GetCharacterToProtect)
          (:then
            (bind _isdead_2 (Default|IsDead _charactertoprotect))
            (if _isdead_2
              (CallFunction|CompleteMission false :!label _label)
              (elif (Utilities|Array|IsEmpty (Variables|Default|GetEnemyToDefeat))
                (CallFunction|CompleteMission true))))
          (:else
            (goto _label)))))
    (else
      (CallFunction|CompleteMission true))))