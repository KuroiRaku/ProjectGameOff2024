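; BP_MissionBook is an interactable item that gives the player a mission.
; On Interact it runs the parent behavior, then, on first use, passes its Mission to BP_CameraController on player controller 0 through SetCurrentMission.
; An IsAdded flag, set only after a successful cast to that controller, stops later interactions from setting the mission again.
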(event EventBeginPlay
  (|CallParentFunction) ; This node is disabled and will not be called.\nDrag off pins to build functionality.
)

(event Collision|EventActorBeginOverlap
  (params (OtherActor :type Actor%20Object%20Reference))
  (|CallParentFunction OtherActor) ; This node is disabled and will not be called.\nDrag off pins to build functionality.
)

(event EventTick
  (params (DeltaSeconds :type Float%20%28single-precision%29))
  (|CallParentFunction DeltaSeconds) ; This node is disabled and will not be called.\nDrag off pins to build functionality.
)

(event EventInteract
  (params (Character :type BP%20Base%20Character%20Object%20Reference))
  (|CallParentFunction Character)
  (if (not (Variables|Default|GetIsAdded))
    (bind _asbp_camera_controller (Utilities|Casting|CastToBP_CameraController (Game|GetPlayerController 0)))
    (Default|SetCurrentMission _asbp_camera_controller (Variables|Default|GetMission))
    (Variables|Default|SetIsAdded true)))

(fn ConstructionScript
  (|CallParentFunction))