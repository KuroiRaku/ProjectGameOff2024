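; Interactable skill book that unlocks a spell slot and configured element, shape, size and speed options on the interacting character's SpellComponent.
; BeginPlay sorts each option array by descending enum value, and Interact prepends each name while unlocking, so each category reads in ascending order.
; For a player character, a non-empty learned list is printed, sent to the book widget, and marks the book as used.
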(event Custom|SortElements
  (bind _element (Variables|Default|GetElement))
  (bind _returnvalue (Utilities|Array|LastIndex _element))
  ;[1 1 1] Elements
  (if (>= (Utilities|Array|Length _element) 2)
    (for _index (range 0 _returnvalue) ; i
      (for _index_2 (range _index _returnvalue) ; ĵ
        (if (> (Math|Conversions|ToInteger(Byte) (Utilities|Array|Get(acopy) _element _index_2)) (Math|Conversions|ToInteger(Byte) (Utilities|Array|Get(acopy) _element _index)))
          (Utilities|Array|Swap _element _index_2 _index))))))

(event Custom|SortShapes
  (bind _shape (Variables|Default|GetShape))
  (bind _returnvalue (Utilities|Array|LastIndex _shape))
  ;[1 1 1] Shapes
  (if (>= (Utilities|Array|Length _shape) 2)
    (for _index (range 0 _returnvalue) ; i
      (for _index_2 (range _index _returnvalue) ; ĵ
        (if (> (Math|Conversions|ToInteger(Byte) (Utilities|Array|Get(acopy) _shape _index_2)) (Math|Conversions|ToInteger(Byte) (Utilities|Array|Get(acopy) _shape _index)))
          (Utilities|Array|Swap _shape _index_2 _index))))))

(event Custom|SortSizes
  (bind _size (Variables|Default|GetSize))
  (bind _returnvalue (Utilities|Array|LastIndex _size))
  ;[1 1 1] Sizes
  (if (>= (Utilities|Array|Length _size) 2)
    (for _index (range 0 _returnvalue) ; i
      (for _index_2 (range _index _returnvalue) ; ĵ
        (if (> (Math|Conversions|ToInteger(Byte) (Utilities|Array|Get(acopy) _size _index_2)) (Math|Conversions|ToInteger(Byte) (Utilities|Array|Get(acopy) _size _index)))
          (Utilities|Array|Swap _size _index_2 _index))))))

(event Custom|SortSpeeds
  (bind _speed (Variables|Default|GetSpeed))
  (bind _returnvalue (Utilities|Array|LastIndex _speed))
  ;[1 1 1] Speeds
  (if (>= (Utilities|Array|Length _speed) 2)
    (for _index (range 0 _returnvalue) ; i
      (for _index_2 (range _index _returnvalue) ; ĵ
        (if (> (Math|Conversions|ToInteger(Byte) (Utilities|Array|Get(acopy) _speed _index_2)) (Math|Conversions|ToInteger(Byte) (Utilities|Array|Get(acopy) _speed _index)))
          (Utilities|Array|Swap _speed _index_2 _index))))))

(event Collision|EventActorBeginOverlap
  (params (OtherActor :type Actor%20Object%20Reference))
  (|CallParentFunction OtherActor) ; This node is disabled and will not be called.\nDrag off pins to build functionality.
)

(event EventTick
  (params (DeltaSeconds :type Float%20%28single-precision%29))
  (|CallParentFunction DeltaSeconds) ; This node is disabled and will not be called.\nDrag off pins to build functionality.
)

(event EventInteract
  (params (Character :type BP%20Base%20Character%20Object%20Reference))
  (bind _spellcomponent (Variables|/Game/Characters/_Common/Blueprint/BP_BaseCharacter.BP_BaseCharacter_C|GetSpellComponent Character))
  (bind _size (Variables|Default|GetSize))
  (bind _spellunlock (Variables|Default|GetSpellUnlock))
  (bind _speed (Variables|Default|GetSpeed))
  (bind _element (Variables|Default|GetElement))
  (bind _shape (Variables|Default|GetShape))
  (bind _spellslotprogression (Variables|/Game/Gameplay/Magic/MagicComponent/BP_SpellComponent.BP_SpellComponent_C|GetSpellSlotProgression _spellcomponent))
  (|CallParentFunction Character)
  (if (not (Variables|Default|GetHaveInteracted))
    (Utilities|IsValid Character
      (:Is%20Valid
        ;[1 1 1] Check Spell Slot to Unlock
        (if (.Value (Utilities|Map|Find _spellslotprogression _spellunlock))
          _
          (else
            (Utilities|Map|Add _spellslotprogression _spellunlock true)))
        ;[1 1 1] Elements
        (if (Utilities|Array|IsEmpty _element)
          _
          (else
            (for _array_element _element
              (Utilities|Map|Add (Variables|/Game/Gameplay/Magic/MagicComponent/BP_SpellComponent.BP_SpellComponent_C|GetElementTypeProgressionMap _spellcomponent) _array_element true)
              (Variables|Default|SetLearnMessageText (Utilities|String|Append (Utilities|String|EnumtoString _array_element) ", " (Variables|Default|GetLearnMessageText))))))
        ;[1 1 1] Shapes
        (if (Utilities|Array|IsEmpty _shape)
          _
          (else
            (for _array_element_2 _shape
              (Utilities|Map|Add (Variables|/Game/Gameplay/Magic/MagicComponent/BP_SpellComponent.BP_SpellComponent_C|GetShapeTypeProgression _spellcomponent) _array_element_2 true)
              (Variables|Default|SetLearnMessageText (Utilities|String|Append (Utilities|String|EnumtoString _array_element_2) ", " (Variables|Default|GetLearnMessageText))))))
        ;[1 1 1] Sizes
        (if (Utilities|Array|IsEmpty _size)
          _
          (else
            (for _array_element_3 _size
              (Utilities|Map|Add (Variables|/Game/Gameplay/Magic/MagicComponent/BP_SpellComponent.BP_SpellComponent_C|GetSizeTypeProgression _spellcomponent) _array_element_3 true)
              (Variables|Default|SetLearnMessageText (Utilities|String|Append (Utilities|String|EnumtoString _array_element_3) ", " (Variables|Default|GetLearnMessageText))))))
        ;[1 1 1] Speeds
        (if (Utilities|Array|IsEmpty _speed)
          _
          (else
            (for _array_element_4 _speed
              (Utilities|Map|Add (Variables|/Game/Gameplay/Magic/MagicComponent/BP_SpellComponent.BP_SpellComponent_C|GetSpeedTypeProgressionMap _spellcomponent) _array_element_4 true)
              (Variables|Default|SetLearnMessageText (Utilities|String|Append (Utilities|String|EnumtoString _array_element_4) ", " (Variables|Default|GetLearnMessageText))))))
        ;[1 1 1] Debug
        (bind _asbp_player_character (Utilities|Casting|CastToBP_PlayerCharacter Character))
        (Utilities|Casting|CastToBP_CameraController (Pawn|GetController _asbp_player_character))
        (if (not (Utilities|Array|IsEmpty (Variables|Default|GetLearnMessageText)))
          (Development|PrintString (Utilities|String|Append "You have learned " (.LeftS (Utilities|String|Split (Variables|Default|GetLearnMessageText) "," "IgnoreCase" "FromEnd"))))
          (Default|UpdateSpellText (Variables|Default|GetBookWidget) (Utilities|Text|ToText(String) (.LeftS (Utilities|String|Split (Variables|Default|GetLearnMessageText) "," "IgnoreCase" "FromEnd"))))
          (Variables|Default|SetHaveInteracted true))))))

(event EventBeginPlay
  (CallFunction|SortElements)
  (CallFunction|SortShapes)
  (CallFunction|SortSizes)
  (CallFunction|SortSpeeds))

(fn ConstructionScript
  (|CallParentFunction))