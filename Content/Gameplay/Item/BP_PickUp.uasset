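; BP_PickUp is a readable book the player can open and close by interacting while nearby.
; The construction script builds a BP_BookWidget from the book ID and its page and spline textures.
; A box overlap with BP_PlayerCharacter gates Interact, which toggles the widget on the viewport with open and close sounds.
; Leaving the box while reading closes the book automatically.
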(event OnComponentBeginOverlap(Box)
  (params (OverlappedComponent :type Primitive%20Component%20Object%20Reference) (OtherActor :type Actor%20Object%20Reference) (OtherComp :type Primitive%20Component%20Object%20Reference) (OtherBodyIndex :type Integer) (bFromSweep :type Boolean) (SweepResult :type Hit%20Result%20Structure%20%28by%20ref%29))
  (Utilities|Casting|CastToBP_PlayerCharacter OtherActor)
  (Variables|Default|SetIsClose? true))

(event OnComponentEndOverlap(Box)
  (params (OverlappedComponent :type Primitive%20Component%20Object%20Reference) (OtherActor :type Actor%20Object%20Reference) (OtherComp :type Primitive%20Component%20Object%20Reference) (OtherBodyIndex :type Integer))
  (Utilities|Casting|CastToBP_PlayerCharacter OtherActor)
  (Variables|Default|SetIsClose? false)
  (if (Variables|Default|GetIsReading?)
    (CallFunction|PutDown)))

(event Custom|TogglePickUp
  (if (Variables|Default|GetIsReading?)
    (CallFunction|PutDown)
    (else
      (CallFunction|PickUp))))

(event Custom|PickUp
  (UserInterface|Viewport|AddtoViewport (Variables|Default|GetBookWidget) 0)
  (Variables|Default|SetIsReading? true)
  (Audio|PlaySound2D "/Game/Assets/SFX/___BOOK_OPEN.___BOOK_OPEN" 1.0 1.0 0.0 0 0))

(event Custom|PutDown
  (Widget|RemovefromParent (Variables|Default|GetBookWidget))
  (Variables|Default|SetIsReading? false)
  (Audio|PlaySound2D "/Game/Assets/SFX/___BOOK_CLOSE.___BOOK_CLOSE" 1.0 1.0 0.0 0 0))

(event EventBeginPlay)

(event Collision|EventActorBeginOverlap
  (params (OtherActor :type Actor%20Object%20Reference)))

(event EventTick
  (params (DeltaSeconds :type Float%20%28single-precision%29)))

(event EventInteract
  (params (Character :type BP%20Base%20Character%20Object%20Reference))
  (if (Variables|Default|GetIsClose?)
    (CallFunction|TogglePickUp)))

(fn ConstructionScript
  (bind _returnvalue (Game|ConstructObjectfromClass "/Game/UI/BP_BookWidget.BP_BookWidget_C" (Variables|Default|GetBookID) (Variables|Default|GetLeftBookTexture) (Variables|Default|GetRightBookTexture) (Variables|Default|GetBookSplineTexture)))
  (Variables|Default|SetBookWidget _returnvalue))

(fn GetObjectName
  (return ""))